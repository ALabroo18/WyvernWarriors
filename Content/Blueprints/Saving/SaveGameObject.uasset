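; Level actor that saves and loads wave progress, player state and GameManager data in one slot, autosaving at BeginPlay.
; BeginPlay caches managers and world actors; SaveGame copies wave number, flamethrower unlock and player start transform into the save object.
; LoadGame restores transform and wave, calls GMLoad on the cached save reference, then resets QTEs, houses and outposts before starting a new wave.
; Enemy cleanup on load is disconnected.
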(event EventBeginPlay
  (Utilities|FlowControl|Sequence
    (:then_0
      (bind _game_state_level (CallFunction|GetGameStateLevel))
      (Variables|Default|SetGame%20State%20Level _game_state_level)
      (bind _asgame_manager (Utilities|Casting|CastToGameManager (Game|GetGameInstance)))
      (Variables|Default|SetAs%20Game%20Manager _asgame_manager)
      (bind _wavemanager (CallFunction|GetWaveManager))
      (Variables|Default|SetWave%20Manager _wavemanager)
      (bind _enemymanager (CallFunction|GetEnemyManager))
      (Variables|Default|SetEnemy%20Manager _enemymanager)
      (bind _asbp_wyvern (Utilities|Casting|CastToBp_wyvern (Game|Player|GetPlayerPawn 0)))
      (Variables|Default|SetAs%20Bp%20Wyvern _asbp_wyvern)
      (bind _returnvalue (Actor|GetActorOfClass "/Game/Blueprints/WaterQTE/WaterQTEManager.WaterQTEManager_C"))
      (Variables|Default|SetWaterQTEManager _returnvalue)
      (bind _returnvalue_2 (Actor|GetActorOfClass "/Game/Blueprints/WeaponQTESpawner/WeaponQTEManager.WeaponQTEManager_C"))
      (Variables|Default|SetWeaponQTEManager _returnvalue_2)
      (bind _outactors (Actor|GetAllActorsOfClass "/Game/LevelDesign/BlockoutPrefabs/WeaponDropOff.WeaponDropOff_C"))
      (Variables|Default|SetWeaponDropOff _outactors)
      (bind _outactors_2 (Actor|GetAllActorsOfClass "/Game/LevelDesign/Prefabs/Houses/VillageHouse1.VillageHouse1_C"))
      (Variables|Default|SetHouses _outactors_2)
      (bind _outactors_3 (Actor|GetAllActorsOfClass "/Game/Blueprints/WeaponQTESpawner/WeaponQTEObject.WeaponQTEObject_C"))
      (Variables|Default|SetWeaponQTEObjects _outactors_3)
      (bind _outactors_4 (Actor|GetAllActorsOfClass "/Game/Blueprints/Outpost/Actor_Outpost.Actor_Outpost_C"))
      (Variables|Default|SetOutposts _outactors_4)
      (bind _asbp_hud (Utilities|Casting|CastToBP_HUD (HUD|GetHUD (Game|GetPlayerController 0))))
      (Variables|Default|SetStat%20HUD (Variables|/Game/Blueprints/UI/HUD/BP_HUD.BP_HUD_C|GetStatHUD _asbp_hud)))
    (:then_1
      (CallFunction|SaveGame))))

(fn ConstructionScript)

(fn SaveGame
  (bind _as_bp_wyvern (Variables|Default|GetAs%20Bp%20Wyvern))
  (Development|PrintString "Autosaving, please do not close the game at this time")
  (Utilities|FlowControl|Sequence
    (:then_0
      ;[0.15 0.15 0.15 0.5] Makes sure save reference exists, if not makes the reference
      (Utilities|IsValid (Variables|Default|GetSaveGameRef)
        (:Is%20Not%20Valid
          (bind _returnvalue (SaveGame|CreateSaveGameObject "/Game/Blueprints/Saving/SaveGame.SaveGame_C"))
          (bind _output_get (Variables|Default|SetSaveGameRef _returnvalue))
          (Default|GetGameManager _output_get (Variables|Default|GetAs%20Game%20Manager)))))
    (:then_1
      ;[0.15 0.15 0.15 0.5] Sequence 1 is all things to be saved
      (Utilities|IsValid (Variables|Default|GetSaveGameRef)
        (:Is%20Valid
          (Utilities|FlowControl|Sequence
            (:then_0
              (Variables|/Game/Blueprints/Saving/SaveGame.SaveGame_C|SetNumOfWaves (Variables|Default|GetSaveGameRef) (Class|GameStateLevel|GetCurrentWaveNumber (Variables|Default|GetGame%20State%20Level)))
              (Default|GMSave (Variables|Default|GetSaveGameRef)))
            (:then_1
              (Variables|/Game/Blueprints/Saving/SaveGame.SaveGame_C|SetHasFlamethrower (Variables|Default|GetSaveGameRef) (Variables|/Game/Blueprints/Characters/Wyvern/Bp_wyvern.Bp_wyvern_C|GetbFlamethrowerUnlocked _as_bp_wyvern))
              (Variables|/Game/Blueprints/Saving/SaveGame.SaveGame_C|SetPlayerLocation (Variables|Default|GetSaveGameRef) (Variables|/Game/Blueprints/Characters/Wyvern/Bp_wyvern.Bp_wyvern_C|GetStartingLocation _as_bp_wyvern)))))))
    (:then_2
      ;[0.15 0.15 0.15 0.5] Saves game to slot
      (SaveGame|SaveGametoSlot (Variables|Default|GetSaveGameRef) (Variables|Default|GetSaveGameSlot))
      (Development|PrintString "Game has been saved."))))

(fn LoadGame
  (bind _waterqtemanager (Variables|Default|GetWaterQTEManager))
  (bind _savegameslot (Variables|Default|GetSaveGameSlot))
  (bind _weaponqtemanager (Variables|Default|GetWeaponQTEManager))
  (bind _returnvalue (SaveGame|DoesSaveGameExist _savegameslot))
  (if _returnvalue
    (Utilities|FlowControl|Sequence
      (:then_0
        ;[0.15 0.15 0.15 0.5] Loads data
        (bind _returnvalue_2 (SaveGame|LoadGamefromSlot _savegameslot))
        (bind _assave_game (Utilities|Casting|CastToSaveGame _returnvalue_2))
        (Utilities|FlowControl|Sequence
          (:then_0
            (Transformation|SetActorTransform (Variables|Default|GetAs%20Bp%20Wyvern) (Variables|/Game/Blueprints/Saving/SaveGame.SaveGame_C|GetPlayerLocation _assave_game)))
          (:then_1
            (Class|GameStateLevel|SetCurrentWaveNumber (Variables|Default|GetGame%20State%20Level) (Variables|/Game/Blueprints/Saving/SaveGame.SaveGame_C|GetNumOfWaves _assave_game))
            (Development|PrintString (Utilities|String|ToString(Integer) (Variables|/Game/Blueprints/Saving/SaveGame.SaveGame_C|GetNumOfWaves _assave_game)))
            (Default|GMLoad (Variables|Default|GetSaveGameRef)))
          (:then_2
            (Utilities|Time|ClearandInvalidateTimerbyHandle (Variables|/Game/Blueprints/WaterQTE/WaterQTEManager.WaterQTEManager_C|GetWaterEventHandle _waterqtemanager))
            (Utilities|Time|ClearandInvalidateTimerbyHandle (Variables|/Game/Blueprints/WeaponQTESpawner/WeaponQTEManager.WeaponQTEManager_C|GetWeaponQTEHandle _weaponqtemanager))
            (Utilities|FlowControl|Sequence
              (:then_0
                (for _array_element (Variables|Default|GetWeaponDropOff)
                  (Utilities|Time|ClearandInvalidateTimerbyHandle (Variables|/Game/LevelDesign/BlockoutPrefabs/WeaponDropOff.WeaponDropOff_C|GetTimeOutHandle _array_element))))
              (:then_1
                (bind _outactors (Actor|GetAllActorsOfClass "/Game/Blueprints/WaterQTE/WaterQTEObject.WaterQTEObject_C"))
                (for _array_element_2 _outactors
                  (Actor|DestroyActor _array_element_2)))
              (:then_2
                (for _array_element_3 (Variables|Default|GetHouses)
                  (Default|HouseColorInitialization _array_element_3)))
              (:then_3
                (for _array_element_4 (Variables|Default|GetWeaponQTEObjects)
                  (Default|ResetQTE _array_element_4)))
              (:then_4
                (for _array_element_5 (Variables|Default|GetOutposts)
                  (Variables|/Game/Blueprints/Outpost/Actor_Outpost.Actor_Outpost_C|SetisLoaded _array_element_5 true)
                  (Default|PlayerCaptureOutpost _array_element_5)))))
          (:then_3
            (Default|WaterEventSpawn _waterqtemanager)
            (Default|WeaponQTESpawn _weaponqtemanager)
            (bind _asbp_hud (Utilities|Casting|CastToBP_HUD (HUD|GetHUD (Game|GetPlayerController 0))))
            (Widget|Panel|ClearChildren (Variables|/Game/Blueprints/UI/HUD/WBP_StatHUD.WBP_StatHUD_C|GetScrollBox_0 (Variables|/Game/Blueprints/UI/HUD/BP_HUD.BP_HUD_C|GetStatHUD _asbp_hud)))
            (Class|WaveManagerComponent|NewWave (Variables|Default|GetWave%20Manager)))))
      (:then_1
        (Development|PrintString "Loaded Game")))
    (else
      ;[0.15 0.15 0.15 0.5] Saves if no save data has been made yet
      (SaveGame|SaveGametoSlot (Variables|Default|GetSaveGameRef) _savegameslot))))