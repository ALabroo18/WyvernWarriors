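; Save manager actor that autosaves and loads wave and level-completion progress for the tutorial, three island levels and main menu.
; BeginPlay maps the level name to an enum, caches managers, runs a delayed load/save (reversed in the menu), and binds saving to final-wave completion.
; SaveGame writes or resets the slot; LoadGame restores GameManager data, wave state and menu completion count.
; Disconnected in-place level reset logic remains unused.
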(event Custom|SaveOnFinalWave
  (params (bIsFinalWave :type Boolean))
  (if bIsFinalWave
    (CallFunction|SaveGame)))

(event EventBeginPlay
  (Utilities|FlowControl|Sequence
    (:then_0
      ;[0.15 0.15 0.15 0.5] Sets the level enum to the correct level
      (bind _returnvalue (Game|GetCurrentLevelName true))
      (bind _output_get (Variables|Default|SetCurrentLevel _returnvalue))
      (if (Utilities|Enum|Equal(Enum) _output_get "IslandLevel")
        (Variables|Default|SetLevelNumberEnum "NewEnumerator0")
        (Development|PrintString "In level 1")
        (elif (Utilities|Enum|Equal(Enum) _output_get "IslandLevel2")
          (Variables|Default|SetLevelNumberEnum "NewEnumerator1")
          (Development|PrintString "In level 2")
          (elif (Utilities|Enum|Equal(Enum) _output_get "IslandLevel3")
            (Variables|Default|SetLevelNumberEnum "NewEnumerator2")
            (Development|PrintString "In level 3")
            (elif (Utilities|Enum|Equal(Enum) _output_get "MainMenu")
              (Variables|Default|SetLevelNumberEnum "NewEnumerator3")
              (Development|PrintString "In MainMenu")
              (elif (Utilities|Enum|Equal(Enum) _output_get "TutLevel")
                (Variables|Default|SetLevelNumberEnum "NewEnumerator4")
                (Development|PrintString "In Tutorial Level")))))))
    (:then_1
      (switch Utilities|FlowControl|Switch|SwitchonCurrentLevelEnum (Variables|Default|GetLevelNumberEnum)
        (:NewEnumerator0
          (bind _wavemanager (CallFunction|GetWaveManager :!label _label))
          (Variables|Managers|SetWave%20Manager _wavemanager)
          (bind _enemymanager (CallFunction|GetEnemyManager))
          (Variables|Managers|SetEnemy%20Manager _enemymanager))
        (:NewEnumerator1
          (goto _label))
        (:NewEnumerator2
          (goto _label))
        (:NewEnumerator3
          _))
      (bind _game_state_level (CallFunction|GetGameStateLevel))
      (Variables|Managers|SetGame%20State%20Level _game_state_level)
      (bind _asgame_manager (Utilities|Casting|CastToGameManager (Game|GetGameInstance)))
      (Variables|Managers|SetAs%20Game%20Manager _asgame_manager)
      (bind _asbp_wyvern (Utilities|Casting|CastToBp_wyvern (Game|Player|GetPlayerPawn 0)))
      (Variables|Default|SetAs%20Bp%20Wyvern _asbp_wyvern)
      (bind _eventbus (CallFunction|GetEventBus))
      (EventDispatchers|BindEventtoOnWaveComplete _eventbus (delegate Custom|SaveOnFinalWave)))
    (:then_2
      (bind _returnvalue_2 (SaveGame|LoadGamefromSlot (Variables|Default|GetSaveGameSlot)))
      (bind _assave_game (Utilities|Casting|CastToSaveGame _returnvalue_2))
      (Variables|Default|SetSaveGameRef _assave_game))
    (:then_3
      ;[0.15 0.15 0.15 0.5] Saves game in MainMenu (when player opens the game) and loads the save data on level load so that the saved data doesnt get overriden, then saves and starts autosaving
      (switch Utilities|FlowControl|Switch|SwitchonCurrentLevelEnum (Variables|Default|GetLevelNumberEnum)
        (:NewEnumerator0
          (Utilities|FlowControl|Delay 0.5 :!label _label_2)
          (CallFunction|LoadGame)
          (Utilities|FlowControl|Delay 1.0)
          (CallFunction|SaveGame))
        (:NewEnumerator1
          (goto _label_2))
        (:NewEnumerator2
          (goto _label_2))
        (:NewEnumerator3
          (Utilities|FlowControl|Delay 0.5)
          (CallFunction|SaveGame)
          (Utilities|FlowControl|Delay 0.5)
          (CallFunction|LoadGame))
        (:NewEnumerator4
          (goto _label_2))))))

(fn ConstructionScript)

(fn SaveGame
  (bind _game_state_level (Variables|Managers|GetGame%20State%20Level))
  (bind _game_state_level_2 (Variables|Managers|GetGame%20State%20Level))
  (bind _game_state_level_3 (Variables|Managers|GetGame%20State%20Level))
  (bind _game_state_level_4 (Variables|Managers|GetGame%20State%20Level))
  (bind _returnvalue (Class|GameStateLevel|GetCurrentWaveNumber _game_state_level_4))
  (bind _returnvalue_2 (Class|GameStateLevel|GetCurrentWaveNumber _game_state_level))
  (bind _returnvalue_3 (Class|GameStateLevel|GetCurrentWaveNumber _game_state_level_2))
  (bind _returnvalue_4 (Class|GameStateLevel|GetCurrentWaveNumber _game_state_level_3))
  (bind _returnvalue_5 (== _returnvalue_2 3))
  (Development|PrintString "Autosaving, please do not close the game at this time")
  (if (Variables|Default|GetisReset)
    ;[0.15 0.15 0.15 0.5] Resets game progress
    (Utilities|FlowControl|Sequence
      (:then_0
        ;;[0.15 0.15 0.15 0.5] Makes sure theres a save game reference
        (Utilities|IsValid (Variables|Default|GetSaveGameRef)
          (:Is%20Not%20Valid
            (bind _returnvalue_6 (SaveGame|CreateSaveGameObject "/Game/Blueprints/Saving/SaveGame.SaveGame_C"))
            (bind _output_get (Variables|Default|SetSaveGameRef _returnvalue_6))
            (Default|GetGameManager _output_get (Variables|Managers|GetAs%20Game%20Manager)))))
      (:then_1
        (Variables|/Game/Blueprints/Saving/SaveGame.SaveGame_C|SetCurrentWaveNumberL1 (Variables|Default|GetSaveGameRef) 0)
        (Variables|/Game/Blueprints/Saving/SaveGame.SaveGame_C|SetCurrentWaveNumberL2 (Variables|Default|GetSaveGameRef) 0)
        (Variables|/Game/Blueprints/Saving/SaveGame.SaveGame_C|SetCurrentWaveNumberL3 (Variables|Default|GetSaveGameRef) 0)
        (Variables|/Game/Blueprints/Saving/SaveGame.SaveGame_C|SetLevel1Complete (Variables|Default|GetSaveGameRef) false)
        (Variables|/Game/Blueprints/Saving/SaveGame.SaveGame_C|SetLevel2Complete (Variables|Default|GetSaveGameRef) false)
        (Variables|/Game/Blueprints/Saving/SaveGame.SaveGame_C|SetLevel3Complete (Variables|Default|GetSaveGameRef) false)
        (Variables|/Game/Blueprints/Saving/SaveGame.SaveGame_C|SetTutorialComplete (Variables|Default|GetSaveGameRef) false)
        (Variables|/Game/Blueprints/Saving/SaveGame.SaveGame_C|SetCurrentLevel (Variables|Default|GetSaveGameRef) "MainMenu"))
      (:then_2
        (SaveGame|SaveGametoSlot (Variables|Default|GetSaveGameRef) (Variables|Default|GetSaveGameSlot))
        (Development|PrintString "Game has been saved.")))
    (else
      (Utilities|FlowControl|Sequence
        (:then_0
          ;[0.15 0.15 0.15 0.5] Makes sure save reference exists, if not makes the reference
          (Utilities|IsValid (Variables|Default|GetSaveGameRef)
            (:Is%20Not%20Valid
              (bind _returnvalue_7 (SaveGame|CreateSaveGameObject "/Game/Blueprints/Saving/SaveGame.SaveGame_C"))
              (bind _output_get_2 (Variables|Default|SetSaveGameRef _returnvalue_7))
              (Default|GetGameManager _output_get_2 (Variables|Managers|GetAs%20Game%20Manager)))))
        (:then_1
          ;[0.15 0.15 0.15 0.5] Sequence 1 is all things to be saved
          (Utilities|IsValid (Variables|Default|GetSaveGameRef)
            (:Is%20Valid
              (Variables|/Game/Blueprints/Saving/SaveGame.SaveGame_C|SetCurrentLevel (Variables|Default|GetSaveGameRef) (Variables|Default|GetCurrentLevel))
              (Default|GMSave (Variables|Default|GetSaveGameRef))
              (switch Utilities|FlowControl|Switch|SwitchonCurrentLevelEnum (Variables|Default|GetLevelNumberEnum)
                (:NewEnumerator0
                  (if (== _returnvalue 2)
                    (Variables|/Game/Blueprints/Saving/SaveGame.SaveGame_C|SetCurrentWaveNumberL1 (Variables|Default|GetSaveGameRef) _returnvalue)
                    (else
                      (Variables|/Game/Blueprints/Saving/SaveGame.SaveGame_C|SetCurrentWaveNumberL1 (Variables|Default|GetSaveGameRef) 0)
                      (if _returnvalue_5
                        (Variables|/Game/Blueprints/Saving/SaveGame.SaveGame_C|SetLevel1Complete (Variables|Default|GetSaveGameRef) true)))))
                (:NewEnumerator1
                  (if (== _returnvalue_4 2)
                    (Variables|/Game/Blueprints/Saving/SaveGame.SaveGame_C|SetCurrentWaveNumberL2 (Variables|Default|GetSaveGameRef) _returnvalue_4)
                    (else
                      (Variables|/Game/Blueprints/Saving/SaveGame.SaveGame_C|SetCurrentWaveNumberL2 (Variables|Default|GetSaveGameRef) 0)
                      (if _returnvalue_5
                        (Variables|/Game/Blueprints/Saving/SaveGame.SaveGame_C|SetLevel2Complete (Variables|Default|GetSaveGameRef) true)))))
                (:NewEnumerator2
                  (if (== _returnvalue_3 2)
                    (Variables|/Game/Blueprints/Saving/SaveGame.SaveGame_C|SetCurrentWaveNumberL3 (Variables|Default|GetSaveGameRef) _returnvalue_3)
                    (else
                      (Variables|/Game/Blueprints/Saving/SaveGame.SaveGame_C|SetCurrentWaveNumberL3 (Variables|Default|GetSaveGameRef) 0)
                      (if _returnvalue_5
                        (Variables|/Game/Blueprints/Saving/SaveGame.SaveGame_C|SetLevel3Complete (Variables|Default|GetSaveGameRef) true)))))))))
        (:then_2
          (if (Variables|Default|GetisLevelOver)
            (Variables|Default|SetisLevelOver false)
            (switch Utilities|FlowControl|Switch|SwitchonCurrentLevelEnum (Variables|Default|GetLevelNumberEnum)
              (:NewEnumerator0
                (Variables|/Game/Blueprints/Saving/SaveGame.SaveGame_C|SetLevel1Complete (Variables|Default|GetSaveGameRef) true))
              (:NewEnumerator1
                (Variables|/Game/Blueprints/Saving/SaveGame.SaveGame_C|SetLevel2Complete (Variables|Default|GetSaveGameRef) true))
              (:NewEnumerator2
                (Variables|/Game/Blueprints/Saving/SaveGame.SaveGame_C|SetLevel3Complete (Variables|Default|GetSaveGameRef) true))
              (:NewEnumerator4
                (Variables|/Game/Blueprints/Saving/SaveGame.SaveGame_C|SetTutorialComplete (Variables|Default|GetSaveGameRef) true)))))
        (:then_3
          ;;[0.15 0.15 0.15 0.5] Saves game to slot
          (SaveGame|SaveGametoSlot (Variables|Default|GetSaveGameRef) (Variables|Default|GetSaveGameSlot))
          (Development|PrintString "Game has been saved."))))))

(fn LoadGame
  (bind _savegameslot (Variables|Default|GetSaveGameSlot))
  (bind _returnvalue (SaveGame|DoesSaveGameExist _savegameslot))
  (if _returnvalue
    (Utilities|FlowControl|Sequence
      (:then_0
        ;[0.15 0.15 0.15 0.5] Loads data
        (bind _returnvalue_2 (SaveGame|LoadGamefromSlot _savegameslot))
        (bind _assave_game (Utilities|Casting|CastToSaveGame _returnvalue_2))
        (switch Utilities|FlowControl|Switch|SwitchonCurrentLevelEnum (Variables|Default|GetLevelNumberEnum)
          (:NewEnumerator0
            (if (== (Variables|/Game/Blueprints/Saving/SaveGame.SaveGame_C|GetCurrentWaveNumberL1 _assave_game) 3)
              (bind _output_get (Variables|/Game/Blueprints/Saving/SaveGame.SaveGame_C|SetCurrentWaveNumberL1 _assave_game (- (Variables|/Game/Blueprints/Saving/SaveGame.SaveGame_C|GetCurrentWaveNumberL1 _assave_game) 1)))
              (Class|GameStateLevel|SetCurrentWaveNumber (Variables|Managers|GetGame%20State%20Level) _output_get)
              (bind _asbp_hud (Utilities|Casting|CastToBP_HUD (HUD|GetHUD (Game|GetPlayerController 0)) :!label _label))
              (Widget|Panel|ClearChildren (Variables|/Game/Blueprints/UI/HUD/WBP_StatHUD.WBP_StatHUD_C|GetScrollBox_0 (Variables|/Game/Blueprints/UI/HUD/BP_HUD.BP_HUD_C|GetStatHUD _asbp_hud)))
              (Class|WaveManagerComponent|WaveCompleted (Variables|Managers|GetWave%20Manager))))
          (:NewEnumerator1
            (if (== (Variables|/Game/Blueprints/Saving/SaveGame.SaveGame_C|GetCurrentWaveNumberL2 _assave_game) 3)
              (bind _output_get_2 (Variables|/Game/Blueprints/Saving/SaveGame.SaveGame_C|SetCurrentWaveNumberL2 _assave_game (- (Variables|/Game/Blueprints/Saving/SaveGame.SaveGame_C|GetCurrentWaveNumberL2 _assave_game) 1)))
              (Class|GameStateLevel|SetCurrentWaveNumber (Variables|Managers|GetGame%20State%20Level) _output_get_2)
              (goto _label)
              (else
                _)))
          (:NewEnumerator2
            (if (== (Variables|/Game/Blueprints/Saving/SaveGame.SaveGame_C|GetCurrentWaveNumberL3 _assave_game) 3)
              (bind _output_get_3 (Variables|/Game/Blueprints/Saving/SaveGame.SaveGame_C|SetCurrentWaveNumberL3 _assave_game (- (Variables|/Game/Blueprints/Saving/SaveGame.SaveGame_C|GetCurrentWaveNumberL3 _assave_game) 1)))
              (Class|GameStateLevel|SetCurrentWaveNumber (Variables|Managers|GetGame%20State%20Level) _output_get_3)
              (goto _label)
              (else
                _)))
          (:NewEnumerator3
            (if (Variables|/Game/Blueprints/Saving/SaveGame.SaveGame_C|GetLevel3Complete _assave_game)
              (Variables|Default|SetnumOfLevelsCompleted 3)
              (elif (Variables|/Game/Blueprints/Saving/SaveGame.SaveGame_C|GetLevel2Complete _assave_game)
                (Variables|Default|SetnumOfLevelsCompleted 2)
                (elif (Variables|/Game/Blueprints/Saving/SaveGame.SaveGame_C|GetLevel1Complete _assave_game)
                  (Variables|Default|SetnumOfLevelsCompleted 1)
                  (elif (Variables|/Game/Blueprints/Saving/SaveGame.SaveGame_C|GetTutorialComplete _assave_game)
                    (Variables|Default|SetnumOfLevelsCompleted 0)
                    (else
                      (Variables|Default|SetnumOfLevelsCompleted -1)
                      (Development|PrintString "TUTORIAL ISNT COMPLETED")))))))
          (:NewEnumerator4
            _))
        (Default|GMLoad _assave_game))
      (:then_1
        (Development|PrintString "Loaded Game")))
    (else
      ;[0.15 0.15 0.15 0.5] Saves if no save data has been made yet
      (CallFunction|SaveGame))))