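; SaveGame object that stores the player's customization index and unlocked color array.
; GetGameManager caches a GameManager reference, which GMSave and GMLoad check for validity before use.
; GMSave pulls the values from the manager's SendSaveData, and GMLoad pushes them back through ReceiveSaveData.
; A PlayerLocation variable is declared but unused.
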(fn GMSave
  (bind _game_manager (Variables|References|GetGame%20Manager)
    (:then
      (bind (_custindex _colorarray) (Default|SendSaveData _game_manager))
      (Variables|Customization|SetwCustomIndex _custindex)
      (Variables|Customization|SetunlockedColors _colorarray))
    (:else)))

(fn GMLoad
  (bind _game_manager (Variables|References|GetGame%20Manager)
    (:then
      (Default|ReceiveSaveData _game_manager (Variables|Customization|GetwCustomIndex) (Variables|Customization|GetunlockedColors)))
    (:else)))

(fn GetGameManager
  (params (gameManager :type Game%20Manager%20Object%20Reference))
  (Variables|References|SetGame%20Manager gameManager))