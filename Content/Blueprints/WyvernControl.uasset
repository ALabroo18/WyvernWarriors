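; Player controller for the wyvern, handling pause, dash, water pickup and wave cutscenes.
; Inputs refresh keyboard/gamepad detection; dash runs timers on AC_WyvernDash, and dash and pickup set tutorial flags.
; Timer-chained camera fades show a random captured outpost with input disabled, starting after BeginPlay, which also binds the event bus's new-wave event.
; Fireball, flamethrower and dodge events are empty, their old logic left disconnected.
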(event Input|EnhancedActionEvents|EnhancedInputActionIA_FireBall
  (params (ActionValue :type Boolean) (ElapsedSeconds :type Float%20%28double-precision%29) (TriggeredSeconds :type Float%20%28double-precision%29) (InputAction :type Input%20Action%20Object%20Reference :default "/Game/Blueprints/Inputs/IA_FireBall.IA_FireBall"))
  ;[0.15 0.15 0.15 0.5] Fireball Attack
)

(event Input|EnhancedActionEvents|EnhancedInputActionIA_FlameThrower
  (params (ActionValue :type Boolean) (ElapsedSeconds :type Float%20%28double-precision%29) (TriggeredSeconds :type Float%20%28double-precision%29) (InputAction :type Input%20Action%20Object%20Reference :default "/Game/Blueprints/Inputs/IA_FlameThrower.IA_FlameThrower"))
  ;[0.15 0.15 0.15 0.5] Flamethrower and WaterQTE/Flamethrower FOV lil buggy, will fix -Adrian
)

(event Input|EnhancedActionEvents|EnhancedInputActionIA_Dash
  (params (ActionValue :type Boolean) (ElapsedSeconds :type Float%20%28double-precision%29) (TriggeredSeconds :type Float%20%28double-precision%29) (InputAction :type Input%20Action%20Object%20Reference :default "/Game/Blueprints/Inputs/IA_Dash.IA_Dash"))
  ;[0.15 0.15 0.15 0.5] New Dash Mechanic
  (Utilities|FlowControl|FlipFlop
    (:A
      (CallFunction|InputDetection)
      (if true
        (if (> (Variables|Default|GetStaminaMeter) 0)
          (if (not (Variables|Default|GetbisDoingAction))
            (if (not (Variables|Default|GetisDashing))
              (Variables|Default|SetbisDoingAction true)
              (Variables|Default|SetisDashing true)
              (Utilities|Time|SetTimerbyFunctionName (Actor|GetComponentbyClass (Variables|Default|GetWyvernPlayer) "/Game/Blueprints/Characters/Wyvern/WyvernComponents/AC_WyvernDash.AC_WyvernDash_C") "DashSetVelocity" 0.016 true)))
          (else
            (CallFunction|TurnOffDash)
            (Variables|Default|SetStaminaMeter 500)))))
    (:B
      (CallFunction|TurnOffDash)
      ;;[0.15 0.15 0.15 0.5] Need to revise this later
      (Utilities|Time|SetTimerbyFunctionName (Actor|GetComponentbyClass (Variables|Default|GetWyvernPlayer) "/Game/Blueprints/Characters/Wyvern/WyvernComponents/AC_WyvernDash.AC_WyvernDash_C") "ResetStamina" 0.5 true))))

(event Input|EnhancedActionEvents|EnhancedInputActionIA_WyvernDodge
  (params (ActionValue :type Boolean) (ElapsedSeconds :type Float%20%28double-precision%29) (TriggeredSeconds :type Float%20%28double-precision%29) (InputAction :type Input%20Action%20Object%20Reference :default "/Game/Blueprints/Inputs/IA_WyvernDodge.IA_WyvernDodge"))
  ;[0.15 0.15 0.15 0.5] Dodge Left
)

(event Input|EnhancedActionEvents|EnhancedInputActionIA_WyvernDodge
  (params (ActionValue :type Boolean) (ElapsedSeconds :type Float%20%28double-precision%29) (TriggeredSeconds :type Float%20%28double-precision%29) (InputAction :type Input%20Action%20Object%20Reference :default "/Game/Blueprints/Inputs/IA_WyvernDodge.IA_WyvernDodge"))
  ;[0.15 0.15 0.15 0.5] Dodge Right
)

(event Input|EnhancedActionEvents|EnhancedInputActionIA_Pickup_DropOffWaterQTE
  (params (ActionValue :type Boolean) (ElapsedSeconds :type Float%20%28double-precision%29) (TriggeredSeconds :type Float%20%28double-precision%29) (InputAction :type Input%20Action%20Object%20Reference :default "/Game/Blueprints/Inputs/IA_Pickup_DropOffWaterQTE.IA_Pickup_DropOffWaterQTE"))
  (bind _tutorialmanagerinst (Variables|Default|GetTutorialManagerInst))
  (bind _wyvernplayer (Variables|Default|GetWyvernPlayer))
  ;[0.15 0.15 0.15 0.5] How you grab water from water sources
  (:Started
    (CallFunction|InputDetection)
    (if (Variables|/Game/Blueprints/Characters/Wyvern/Bp_wyvern.Bp_wyvern_C|GetInWater (Variables|Default|GetWyvernPlayer))
      (Variables|/Game/Blueprints/Characters/Wyvern/Bp_wyvern.Bp_wyvern_C|SetHasWater (Variables|Default|GetWyvernPlayer) true)
      (Variables|/Game/Blueprints/Characters/Wyvern/Bp_wyvern.Bp_wyvern_C|SetWaterTimerRemaining _wyvernplayer (Variables|/Game/Blueprints/Characters/Wyvern/Bp_wyvern.Bp_wyvern_C|GetWaterTimerMax (Variables|Default|GetWyvernPlayer)))
      (Rendering|SetVisibility (Variables|/Game/Blueprints/Characters/Wyvern/Bp_wyvern.Bp_wyvern_C|GetWaterQTEIcon _wyvernplayer) true false)
      ;[0.15 0.15 0.15 0.5] Gets rid of the pick up water instructions
      (bind _asbp_hud (Utilities|Casting|CastToBP_HUD (HUD|GetHUD (Game|GetPlayerController 0))))
      (Default|PickUpWaterClear (Variables|/Game/Blueprints/UI/HUD/BP_HUD.BP_HUD_C|GetStatHUD _asbp_hud))
      (Utilities|IsValid _tutorialmanagerinst
        (:Is%20Valid
          (Variables|/Game/Blueprints/Tutorial/BP_TutorialManager.BP_TutorialManager_C|SetbPlayerDidPickupWater _tutorialmanagerinst true) ; Tutorial Variable
        )))))

(event Input|EnhancedActionEvents|EnhancedInputActionIA_PauseGame
  (params (ActionValue :type Boolean) (ElapsedSeconds :type Float%20%28double-precision%29) (TriggeredSeconds :type Float%20%28double-precision%29) (InputAction :type Input%20Action%20Object%20Reference :default "/Game/Blueprints/Inputs/IA_PauseGame.IA_PauseGame"))
  (bind _returnvalue (Game|GetPlayerController 0))
  ;[0.15 0.15 0.15 0.5] PauseMenu
  (CallFunction|InputDetection)
  (if (not (Variables|/Game/Blueprints/Characters/Wyvern/Bp_wyvern.Bp_wyvern_C|GetisPausedMenuOpen (Variables|Default|GetWyvernPlayer)))
    (Variables|/Game/Blueprints/Characters/Wyvern/Bp_wyvern.Bp_wyvern_C|SetisPausedMenuOpen (Variables|Default|GetWyvernPlayer) true)
    (bind _returnvalue_2 (UserInterface|CreateWidget "/Game/Blueprints/UI/MenuScreen/WB_PauseMenu.WB_PauseMenu_C" _returnvalue))
    (bind _output_get (Variables|/Game/Blueprints/Characters/Wyvern/Bp_wyvern.Bp_wyvern_C|SetPaused%20Menu%20WIdget (Variables|Default|GetWyvernPlayer) _returnvalue_2))
    (UserInterface|Viewport|AddtoViewport _output_get 0)
    (Input|SetInputModeGameandUI _returnvalue (Variables|/Game/Blueprints/Characters/Wyvern/Bp_wyvern.Bp_wyvern_C|GetPaused%20Menu%20WIdget (Variables|Default|GetWyvernPlayer)) "DoNotLock" true false)
    (Variables|/Script/Engine.PlayerController|SetbShowMouseCursor _returnvalue true)
    (Input|DisableInput (Variables|Default|GetWyvernPlayer) _returnvalue)
    (Game|SetGamePaused true)
    (else
      (Variables|/Game/Blueprints/Characters/Wyvern/Bp_wyvern.Bp_wyvern_C|SetisPausedMenuOpen (Variables|Default|GetWyvernPlayer) false)
      (Widget|RemovefromParent (Variables|/Game/Blueprints/Characters/Wyvern/Bp_wyvern.Bp_wyvern_C|GetPaused%20Menu%20WIdget (Variables|Default|GetWyvernPlayer)))
      (Game|SetGamePaused false)
      (Input|SetInputModeGameOnly _returnvalue false)
      (Variables|/Script/Engine.PlayerController|SetbShowMouseCursor _returnvalue false))))

(event EventBeginPlay
  ;[5.536 0.05838 0.0633 0.5] Allows inputs from bp_wyvern to be called here
  (Utilities|FlowControl|Sequence
    (:then_0
      (bind _asbp_wyvern (Utilities|Casting|CastToBp_wyvern (Pawn|GetControlledPawn)))
      (Variables|Default|SetWyvernPlayer _asbp_wyvern)
      ;[0.15 0.15 0.15 0.5] Set TutorialManager Instance to handle step input checking
      (bind _returnvalue (Actor|GetActorOfClass "/Game/Blueprints/Tutorial/BP_TutorialManager.BP_TutorialManager_C"))
      (Variables|Default|SetTutorialManagerInst _returnvalue)
      (Variables|Camera|SetPlayerCamera (Game|GetPlayerCameraManager 0))
      (bind _eventbus (CallFunction|GetEventBus))
      (EventDispatchers|BindEventtoOnNewWave _eventbus (EventDispatchers|CreateEvent :!event StartWaveCameraFade))
      (bind _wavemanager (CallFunction|GetWaveManager))
      (Variables|Default|SetWave%20Manager _wavemanager)
      (Utilities|FlowControl|Delay 5.0)
      (Camera|StartWaveCameraFade false))))

(fn ConstructionScript)

(fn HideQTE)

(fn DashLoop)

(fn InputDetection
  (if (not (!= (Variables|Default|GetisKBMInput) (Utilities|String|Contains (Utilities|String|EnumtoString (.PrimaryDeviceType (Utilities|Struct|BreakHardwareDeviceIdentifier (Class|InputDeviceSubsystem|GetMostRecentlyUsedHardwareDevice (|InputDeviceSubsystem))))) "gamepad")))
    (Variables|Default|SetisKBMInput (not (Variables|Default|GetisKBMInput)))
    (bind _asbp_wyvern (Utilities|Casting|CastToBp_wyvern (Game|Player|GetPlayerPawn 0)))
    (Default|ChooseInputType _asbp_wyvern)
    (bind _asgame_manager (Utilities|Casting|CastToGameManager (Game|GetGameInstance)))
    (Default|CallInputChange _asgame_manager (Variables|Default|GetisKBMInput))))

(fn TurnOffDash
  (bind _tutorialmanagerinst (Variables|Default|GetTutorialManagerInst))
  (Utilities|Time|ClearTimerbyFunctionName (Actor|GetComponentbyClass (Variables|Default|GetWyvernPlayer) "/Game/Blueprints/Characters/Wyvern/WyvernComponents/AC_WyvernDash.AC_WyvernDash_C") "DashSetVelocity")
  (Variables|Default|SetbisDoingAction false)
  (Variables|Default|SetisDashing false)
  (Utilities|IsValid _tutorialmanagerinst
    (:Is%20Valid
      (Variables|/Game/Blueprints/Tutorial/BP_TutorialManager.BP_TutorialManager_C|SetbPlayerDidDash _tutorialmanagerinst true) ; Tutorial Variable
    )))

(fn StartWaveCameraFade
  (params (bIsFinalWave :type Boolean))
  (if (not bIsFinalWave)
    (Input|DisableInput (Variables|Default|GetWyvernPlayer) self)
    (Default|CallOnCutsceneEvent true)
    (CameraFades|StartCameraFade :self (Variables|Camera|GetPlayerCamera) :ToAlpha 1.0 :Duration (Variables|Camera|GetWaveFadeDuration) :bHoldWhenFinished true)
    (Utilities|Time|SetTimerbyEvent (EventDispatchers|CreateEvent :!event MoveCameratoOutpost) (+ 0.5 (Variables|Camera|GetWaveFadeDuration)))))

(fn MoveCameratoOutpost
  (bind _returnvalue (Class|WaveManagerComponent|GetRandomCapturedOutpost (Variables|Default|GetWave%20Manager)))
  (Utilities|IsValid (Variables|/Script/WyvernWarriors.Outpost|GetOutpostCamera _returnvalue)
    (:Is%20Valid
      (Game|Player|SetViewTargetwithBlend (Variables|/Script/WyvernWarriors.Outpost|GetOutpostCamera _returnvalue) 0.0 "VTBlend_Linear" 0.0 false)
      (CameraFades|StopCameraFade (Variables|Camera|GetPlayerCamera))
      (Utilities|Time|SetTimerbyEvent (EventDispatchers|CreateEvent :!event ReturnWaveCameraFade) (Variables|Camera|GetOutpostViewTime)))
    (:Is%20Not%20Valid
      (Camera|StopCinematics)
      (return))))

(fn ReturnWaveCameraFade
  (CameraFades|StartCameraFade :self (Variables|Camera|GetPlayerCamera) :ToAlpha 1.0 :Duration (Variables|Camera|GetWaveFadeDuration) :bHoldWhenFinished true)
  (Utilities|Time|SetTimerbyEvent (EventDispatchers|CreateEvent :!event ReturnCameratoPlayer) (+ 0.5 (Variables|Camera|GetWaveFadeDuration))))

(fn ReturnCameratoPlayer
  (Game|Player|SetViewTargetwithBlend (Game|Player|GetPlayerPawn 0) 0.0 "VTBlend_Linear" 0.0 false)
  (Camera|StopCinematics))

(fn StopCinematics
  (CameraFades|StopCameraFade (Variables|Camera|GetPlayerCamera))
  (Default|CallOnCutsceneEvent false)
  (Input|EnableInput (Variables|Default|GetWyvernPlayer) self))