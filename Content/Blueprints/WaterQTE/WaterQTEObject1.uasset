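; A timed fire quick-time event actor that the player puts out with water before it burns a house.
; Each Water overlap shrinks FireArea until it is small enough to count as completed, while a QTELength delay triggers failure.
; FireFinished raises or lowers the control meter, updates the HUD, burns a house on failure and restarts WaterQTEManager's spawn timer.
; Tick scales the icon widget by player distance.
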(event OnComponentBeginOverlap(FireArea)
  (params (OverlappedComponent :type Primitive%20Component%20Object%20Reference) (OtherActor :type Actor%20Object%20Reference) (OtherComp :type Primitive%20Component%20Object%20Reference) (OtherBodyIndex :type Integer) (bFromSweep :type Boolean) (SweepResult :type Hit%20Result%20Structure%20%28by%20ref%29))
  (bind _firearea (Variables|Default|GetFireArea))
  (bind _returnvalue (Transformation|GetWorldScale _firearea))
  (bind (_x _y _z) (Math|Vector|BreakVector _returnvalue))
  (bind _aswater (Utilities|Casting|CastToWater OtherActor)
    (:then
      (bind _output_get (Variables|Default|SetWaterObject _aswater))
      (Utilities|IsValid _output_get
        (:Is%20Valid
          (Transformation|SetRelativeScale3D (Variables|Default|GetFireArea) (- (Transformation|GetWorldScale (Variables|Default|GetFireArea)) "1.000000,1.000000,1.000000"))
          (if (Math|Boolean|ORBoolean (<= _x 1.0) (<= _y 1.0) (<= _z 1.0))
            (Variables|Default|SetCompleted true)
            (CallFunction|FireFinished)
            (Actor|DestroyActor)))))
    (:CastFailed
      (Development|PrintString "Hello"))))

(event Custom|SetImg
  (params (Distance :type Float%20%28double-precision%29))
  (bind _output_get (Variables|Default|SetisClose (<= Distance 5e+04)))
  (if _output_get
    (Widget|Transform|SetRenderScale (UserInterface|GetWidget (Variables|Default|GetFireQTEIcon)) (Math|Conversions|ToVector2D(Vector) (Math|Float|MapRangeClamped Distance 5e+04 1.0 2.0 1.0)))))

(event EventBeginPlay
  (bind _returnvalue (Actor|GetActorOfClass "/Game/Blueprints/WaterQTE/WaterQTEManager.WaterQTEManager_C"))
  (Variables|Default|SetWaterEventManager _returnvalue)
  (bind _wavemanager (CallFunction|GetWaveManager))
  (Variables|Default|SetWave%20Management%20Component _wavemanager)
  (bind _asbp_hud (Utilities|Casting|CastToBP_HUD (HUD|GetHUD (Game|GetPlayerController 0))))
  (bind _output_get (Variables|Default|SetStat%20HUD (Variables|/Game/Blueprints/UI/HUD/BP_HUD.BP_HUD_C|GetStatHUD _asbp_hud)))
  (Variables|/Game/Blueprints/UI/HUD/WBP_StatHUD.WBP_StatHUD_C|SetisItBurning _output_get true)
  ;[0.15 0.15 0.15 0.5] Sets how long until fire goes out and player loses points, also sets WaveManager
  (Utilities|FlowControl|Delay (Variables|Default|GetQTELength))
  (Variables|Default|SetCompleted false)
  (CallFunction|FireFinished))

(event EventTick
  (params (DeltaSeconds :type Float%20%28single-precision%29))
  (CallFunction|SetImg (CallFunction|CheckDistance)))

(fn ConstructionScript)

(fn FireFinished
  (bind _stat_hud (Variables|Default|GetStat%20HUD))
  (bind _wave_management_component (Variables|Default|GetWave%20Management%20Component))
  ;[0.15 0.15 0.15 0.5] Comment
  (if (Variables|Default|GetCompleted)
    (Class|WaveManagerComponent|ModifyControlMeterCurrent _wave_management_component 5e+01 false)
    (Variables|/Game/Blueprints/UI/HUD/WBP_StatHUD.WBP_StatHUD_C|SetisItBurning _stat_hud false)
    (Math|Integer|IncrementInt (Variables|/Game/Blueprints/UI/HUD/WBP_StatHUD.WBP_StatHUD_C|GetCurrentWaterQTE _stat_hud)
      (:%20%20
        _))
    (else
      (Class|WaveManagerComponent|ModifyControlMeterCurrent _wave_management_component -5e+01 false)
      (Variables|/Game/Blueprints/UI/HUD/WBP_StatHUD.WBP_StatHUD_C|SetisItBurning _stat_hud true)
      (Default|BurnHouse (Variables|Default|GetWaterEventManager))))
  (Default|TimetoSpawnTimer (Variables|Default|GetWaterEventManager))
  (Actor|DestroyActor)
  (return))

(fn CheckDistance
  (bind _returnvalue (Game|GetPlayerCharacter 0))
  (Utilities|IsValid _returnvalue
    (:Is%20Valid
      (bind _output_get (Variables|Default|SetDistance%20to%20Player (Math|Vector|Distance(Vector) (Transformation|GetActorLocation self) (Transformation|GetActorLocation _returnvalue))))
      (return _output_get))))