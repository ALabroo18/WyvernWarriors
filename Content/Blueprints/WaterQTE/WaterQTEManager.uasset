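; Manager for the water quick-time event that sets a random house on fire and alerts the player.
; On BeginPlay it caches the wave management component and waits a random delay, then fires once unless it is the final wave.
; It spawns a WaterQTEObject at a fixed offset from a random "House"-tagged actor, leaving the "Fire" socket lookup unused.
; It then sets the HUD's burning flag and shows a notification popup.
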(event Custom|TimeToSpawnTimer
  ;[0.15 0.15 0.15 0.5] Spawns in Water Event when called
  (Utilities|FlowControl|Delay (Math|Random|RandomFloatinRange 5.0 1e+01))
  (if (not (Variables|/Script/WyvernWarriors.WaveManagerComponent|GetbIsFinalWave (Variables|Default|GetWave%20Management%20Component)))
    (CallFunction|SpawnFireatRandomHouse)))

(event Custom|SpawnFireAtRandomHouse
  ;[0.15 0.15 0.15 0.5] Decides where to spawn QTE; Standin handles telling manager to spawn
  (CallFunction|SpawnFire)
  (CallFunction|TellHUD))

(event EventBeginPlay
  ;[0.15 0.15 0.15 0.5] Starts searching for place to spawn fire and sets wave manager
  (bind _wave_management_component (CallFunction|GetWaveManagementComponent))
  (Variables|Default|SetWave%20Management%20Component _wave_management_component)
  (CallFunction|TimetoSpawnTimer))

(fn ConstructionScript)

(fn SpawnFire
  ;[0.15 0.15 0.15 0.5] Spawns fire on random house with tag "House" at the socket location "Fire"
  (bind _outactors (Actor|GetAllActorswithTag "House"))
  (Utilities|IsValid (Variables|/Script/Engine.Actor|GetRootComponent (Utilities|Array|Get(acopy) _outactors (Math|Random|RandomIntegerinRange 0 (Utilities|Array|LastIndex _outactors))))
    (:Is%20Valid
      (Game|SpawnActorfromClass "/Game/Blueprints/WaterQTE/WaterQTEObject.WaterQTEObject_C" (Math|Conversions|ToTransform(Vector) (+ (Transformation|GetActorLocation (Utilities|Array|Get(acopy) _outactors (Math|Random|RandomIntegerinRange 0 (Utilities|Array|LastIndex _outactors)))) "50.000000,-450.000000,700.000000")) "Undefined" "MultiplyWithRoot" 0 0))
    (:Is%20Not%20Valid
      (Development|PrintString "Hello"))))

(fn TellHUD
  ;[0.15 0.15 0.15 0.5] Tells HUD to tell the player that a Water event is happening
  (bind _asbp_hud (Utilities|Casting|CastToBP_HUD (HUD|GetHUD (Game|GetPlayerController 0))))
  (Variables|/Game/Blueprints/UI/HUD/WBP_StatHUD.WBP_StatHUD_C|SetisItBurning (Variables|/Game/Blueprints/UI/HUD/BP_HUD.BP_HUD_C|GetStatHUD _asbp_hud) true)
  (Default|CreateNotificationPopup (Variables|/Game/Blueprints/UI/HUD/BP_HUD.BP_HUD_C|GetStatHUD _asbp_hud) " 
Put out the raging fire!  
" (Variables|Default|GetBurning%20House%20Image)))