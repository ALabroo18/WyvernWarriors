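; Stand-in actor for a water quick-time event: a fire the player puts out with Water before QTELength runs out.
; Each Water overlap shrinks FireArea until it is small enough to count as completed and the actor is destroyed.
; FireFinished raises the control meter on success or lowers it on timeout, updates StatHUD, notifies the tutorial manager and calls WaterQTEManager's spawn timer.
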(event OnComponentBeginOverlap(FireArea)
  (params (OverlappedComponent :type Primitive%20Component%20Object%20Reference) (OtherActor :type Actor%20Object%20Reference) (OtherComp :type Primitive%20Component%20Object%20Reference) (OtherBodyIndex :type Integer) (bFromSweep :type Boolean) (SweepResult :type Hit%20Result%20Structure%20%28by%20ref%29))
  (bind _firearea (Variables|Default|GetFireArea))
  (bind _returnvalue (Transformation|GetWorldScale _firearea))
  (bind (_x _y _z) (Math|Vector|BreakVector _returnvalue))
  (bind _aswater (Utilities|Casting|CastToWater OtherActor))
  (bind _output_get (Variables|Default|SetWaterObject _aswater))
  (Utilities|IsValid _output_get
    (:Is%20Valid
      (Transformation|SetRelativeScale3D (Variables|Default|GetFireArea) (- (Transformation|GetWorldScale (Variables|Default|GetFireArea)) "1.000000,1.000000,1.000000"))
      (if (Math|Boolean|ORBoolean (<= _x 1.0) (<= _y 1.0) (<= _z 1.0))
        (Variables|Default|SetCompleted true)
        (CallFunction|FireFinished)
        (Actor|DestroyActor)))))

(event EventBeginPlay
  (bind _returnvalue (Actor|GetActorOfClass "/Game/Blueprints/Tutorial/BP_TutorialManager.BP_TutorialManager_C"))
  (Variables|Default|SetTutorialManagerInst _returnvalue)
  (bind _wavemanager (CallFunction|GetWaveManager))
  (Variables|Default|SetWave%20Management%20Component _wavemanager)
  (bind _asbp_hud (Utilities|Casting|CastToBP_HUD (HUD|GetHUD (Game|GetPlayerController 0))))
  (bind _output_get (Variables|Default|SetStat%20HUD (Variables|/Game/Blueprints/UI/HUD/BP_HUD.BP_HUD_C|GetStatHUD _asbp_hud)))
  (Variables|/Game/Blueprints/UI/HUD/WBP_StatHUD.WBP_StatHUD_C|SetisItBurning _output_get true)
  ;[0.15 0.15 0.15 0.5] Sets how long until fire goes out and player loses points, also sets WaveManager
  (Utilities|FlowControl|Delay (Variables|Default|GetQTELength))
  (Variables|Default|SetCompleted false)
  (CallFunction|FireFinished))

(fn ConstructionScript)

(fn FireFinished
  (bind _wave_management_component (Variables|Default|GetWave%20Management%20Component))
  (bind _stat_hud (Variables|Default|GetStat%20HUD))
  (bind _tutorialmanagerinst (Variables|Default|GetTutorialManagerInst))
  ;[0.15 0.15 0.15 0.5] Comment
  (if (Variables|Default|GetCompleted)
    (Class|WaveManagerComponent|ModifyControlMeterCurrent _wave_management_component 5e+01 false)
    (Variables|/Game/Blueprints/UI/HUD/WBP_StatHUD.WBP_StatHUD_C|SetisItBurning _stat_hud false)
    (Math|Integer|IncrementInt (Variables|/Game/Blueprints/UI/HUD/WBP_StatHUD.WBP_StatHUD_C|GetCurrentWaterQTE _stat_hud)
      (:%20%20
        _))
    (else
      (Class|WaveManagerComponent|ModifyControlMeterCurrent _wave_management_component -5e+01 false)
      (Variables|/Game/Blueprints/UI/HUD/WBP_StatHUD.WBP_StatHUD_C|SetisItBurning _stat_hud true)))
  (Default|CheckStepComplete _tutorialmanagerinst)
  (Variables|/Game/Blueprints/Tutorial/BP_TutorialManager.BP_TutorialManager_C|SetbPlayerDidFireball _tutorialmanagerinst true)
  (bind _returnvalue (Actor|GetActorOfClass "/Game/Blueprints/WaterQTE/WaterQTEManager.WaterQTEManager_C"))
  (Default|TimetoSpawnTimer _returnvalue)
  (return))