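; Fire actor for the water QTE, which the player must put out before a level-shortened timer expires.
; Each WaterSpray call shrinks the fire area until it is out, while a looping timer fills the widget icon.
; FireFinished raises the control meter on success, or lowers it and burns a house on failure, updating the HUD.
; It then requests the next event from WaterQTEManager outside the tutorial, which also has no timer.
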(event OnComponentBeginOverlap(FireArea)
  (params (OverlappedComponent :type Primitive%20Component%20Object%20Reference) (OtherActor :type Actor%20Object%20Reference) (OtherComp :type Primitive%20Component%20Object%20Reference) (OtherBodyIndex :type Integer) (bFromSweep :type Boolean) (SweepResult :type Hit%20Result%20Structure%20%28by%20ref%29)))

(event Custom|SetImg
  (params (Distance :type Float%20%28double-precision%29))
  (bind _output_get (Variables|Default|SetisClose (<= Distance 5e+04)))
  (if _output_get
    (Widget|Transform|SetRenderScale (UserInterface|GetWidget (Variables|Default|GetFireQTEIcon)) (Math|Conversions|ToVector2D(Vector) (Math|Float|MapRangeClamped Distance 5e+04 1.0 2.0 1.0)))))

(event Custom|WaterSpray
  (bind _firearea (Variables|Default|GetFireArea))
  (bind _returnvalue (Transformation|GetWorldScale _firearea))
  (bind (_x _y _z) (Math|Vector|BreakVector _returnvalue))
  (Transformation|SetRelativeScale3D (Variables|Default|GetFireArea) (- (Transformation|GetWorldScale (Variables|Default|GetFireArea)) "1.000000,1.000000,1.000000"))
  (if (Math|Boolean|ORBoolean (<= _x 1.0) (<= _y 1.0) (<= _z 1.0))
    (Variables|Default|SetCompleted true)
    (CallFunction|FireFinished)
    (Actor|DestroyActor)))

(event Custom|EndTimer
  ;[0.15 0.15 0.15 0.5] Ends timer
  (Variables|Default|SetCompleted false)
  (CallFunction|FireFinished))

(event EventBeginPlay
  (bind _returnvalue (Actor|GetActorOfClass "/Game/Blueprints/Characters/Wyvern/Bp_wyvern.Bp_wyvern_C"))
  (Variables|Default|SetPlayer _returnvalue)
  (bind _returnvalue_2 (Actor|GetActorOfClass "/Game/Blueprints/WaterQTE/WaterQTEManager.WaterQTEManager_C"))
  (bind _output_get (Variables|Default|SetWaterEventManager _returnvalue_2))
  (bind _wavemanager (CallFunction|GetWaveManager))
  (Variables|Default|SetWave%20Management%20Component _wavemanager)
  (bind _asbp_hud (Utilities|Casting|CastToBP_HUD (HUD|GetHUD (Game|GetPlayerController 0))))
  (bind _output_get_2 (Variables|Default|SetStat%20HUD (Variables|/Game/Blueprints/UI/HUD/BP_HUD.BP_HUD_C|GetStatHUD _asbp_hud)))
  (Variables|/Game/Blueprints/UI/HUD/WBP_StatHUD.WBP_StatHUD_C|SetisItBurning _output_get_2 true)
  ;[0.15 0.15 0.15 0.5] Sets how long until fire goes out and player loses points, also sets WaveManager
  (if (not (Variables|Default|GetisInTutorial))
    (CallFunction|GetWaterUI)
    (bind _output_get_3 (Variables|Default|SetTimerValue (- (Variables|Default|GetQTELength) (* (Variables|/Game/Blueprints/WaterQTE/WaterQTEManager.WaterQTEManager_C|GetLevelNumber _output_get) 5.0))))
    (bind _returnvalue_3 (Utilities|Time|SetTimerbyEvent (delegate Custom|EndTimer) _output_get_3))
    (Variables|Default|SetWaterEventTimer _returnvalue_3)
    (bind _returnvalue_4 (Utilities|Time|SetTimerbyFunctionName 0 "SetWaterIconFill" 0.5 true))
    (Variables|Default|SetFillTimer _returnvalue_4)))

(event EventTick
  (params (DeltaSeconds :type Float%20%28single-precision%29)))

(fn ConstructionScript)

(fn FireFinished
  (bind _stat_hud (Variables|Default|GetStat%20HUD))
  (bind _wave_management_component (Variables|Default|GetWave%20Management%20Component))
  ;[0.15 0.15 0.15 0.5] Comment
  (if (Variables|Default|GetCompleted)
    (Class|WaveManagerComponent|ModifyControlMeterCurrent _wave_management_component 5e+01 false)
    (Variables|/Game/Blueprints/UI/HUD/WBP_StatHUD.WBP_StatHUD_C|SetisItBurning _stat_hud false)
    (Math|Integer|IncrementInt (Variables|/Game/Blueprints/UI/HUD/WBP_StatHUD.WBP_StatHUD_C|GetCurrentWaterQTE _stat_hud)
      (:%20%20
        _))
    (else
      (Class|WaveManagerComponent|ModifyControlMeterCurrent _wave_management_component -5e+01 false)
      (Variables|/Game/Blueprints/UI/HUD/WBP_StatHUD.WBP_StatHUD_C|SetisItBurning _stat_hud true)
      (Default|BurnHouse (Variables|Default|GetWaterEventManager))))
  (if (Variables|Default|GetisInTutorial)
    _
    (else
      (Default|WaterEventSpawn (Variables|Default|GetWaterEventManager))))
  (Actor|DestroyActor)
  (return))

(fn CheckDistance
  (bind _returnvalue (Game|GetPlayerCharacter 0))
  (Utilities|IsValid _returnvalue
    (:Is%20Valid
      (bind _output_get (LocalVariables|SetDistance%20to%20Player (Math|Vector|Distance(Vector) (Transformation|GetActorLocation self) (Transformation|GetActorLocation _returnvalue))))
      (return _output_get))))

(fn SetWaterIconFill
  ;[0.15 0.15 0.15 0.5] Fills the water icon based on current timer
  (if (Utilities|Time|IsTimerActivebyHandle (Variables|Default|GetWaterEventTimer))
    (Variables|/Game/Blueprints/WaterQTE/WaterQTEUI.WaterQTEUI_C|SetFill%20Percent (Variables|Default|GetAs%20Water%20QTEUI) (CallFunction|ConvertTimertoFill (Variables|Default|GetWaterEventTimer)))
    (else
      (Utilities|Time|InvalidateTimerHandle (Variables|Default|GetFillTimer)))))

(fn ConvertTimertoFill
  (params (Handle :type Timer%20Handle%20Structure))
  (return (/ (Class|KismetSystemLibrary|GetTimerElapsedTimeHandle Handle) (Variables|Default|GetTimerValue))))

(fn GetWaterUI
  (bind _aswater_qteui (Utilities|Casting|CastToWaterQTEUI (UserInterface|GetWidget (Variables|Default|GetFireQTEIcon))))
  (Variables|Default|SetAs%20Water%20QTEUI _aswater_qteui))