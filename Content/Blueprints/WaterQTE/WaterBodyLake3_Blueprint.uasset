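; A lake water body Blueprint that detects when the player wyvern enters or leaves the water.
; On begin overlap it starts the water QTE on Bp_wyvern and calls PickUpWater on the BP_HUD stat widget.
; On end overlap it sets the wyvern's InWater flag to false and calls PickUpWaterClear on that widget.
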(event Collision|EventActorBeginOverlap
  (params (OtherActor :type Actor%20Object%20Reference))
  ;[0.15 0.15 0.15 0.5] Detects when player is in water and notifies player bp
  (bind _asbp_wyvern (Utilities|Casting|CastToBp_wyvern OtherActor))
  (Default|StartWaterQTE _asbp_wyvern)
  (bind _asbp_hud (Utilities|Casting|CastToBP_HUD (HUD|GetHUD (Game|GetPlayerController 0))))
  (Default|PickUpWater (Variables|/Game/Blueprints/UI/HUD/BP_HUD.BP_HUD_C|GetStatHUD _asbp_hud)))

(event Collision|EventActorEndOverlap
  (params (OtherActor :type Actor%20Object%20Reference))
  ;[0.15 0.15 0.15 0.5] Detects when player is in water and notifies player bp
  (bind _asbp_wyvern (Utilities|Casting|CastToBp_wyvern OtherActor))
  (Variables|/Game/Blueprints/Characters/Wyvern/Bp_wyvern.Bp_wyvern_C|SetInWater _asbp_wyvern false)
  (bind _asbp_hud (Utilities|Casting|CastToBP_HUD (HUD|GetHUD (Game|GetPlayerController 0))))
  (Default|PickUpWaterClear (Variables|/Game/Blueprints/UI/HUD/BP_HUD.BP_HUD_C|GetStatHUD _asbp_hud)))

(fn ConstructionScript)