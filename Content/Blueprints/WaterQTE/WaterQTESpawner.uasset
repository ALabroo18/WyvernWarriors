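; WaterQTESpawner is a spawn point for the fire-extinguishing WaterQTE event, triggered through SpawnWaterQTEEvent.
; The event spawns a WaterQTEObject at this actor's own transform and prints that transform for debugging.
; It then casts player 0's HUD to BP_HUD, sets IsItBurning on its StatHUD and shows a burning-house popup telling the player to put out the fire.
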(event Custom|SpawnWaterQTEEvent
  ;[0.15 0.15 0.15 0.5] When told to spawn fire by WaterQTEManager, it spawns the WaterQTE at this specific gameobject
  (CallFunction|SpawninWaterQTE)
  (CallFunction|TellHUD))

(fn ConstructionScript)

(fn SpawninWaterQTE
  (bind _returnvalue (Transformation|GetActorTransform))
  (Game|SpawnActorfromClass "/Game/Blueprints/WaterQTE/WaterQTEObject.WaterQTEObject_C" _returnvalue "Undefined" "MultiplyWithRoot" 0 false 0)
  (Development|PrintString (Utilities|String|ToString(Transform) _returnvalue) false))

(fn TellHUD
  ;[0.15 0.15 0.15 0.5] Tells HUD to tell the player that a WaterQTE event is happening
  (bind _asbp_hud (Utilities|Casting|CastToBP_HUD (HUD|GetHUD (Game|GetPlayerController 0))))
  (Variables|Default|SetisItBurning (Variables|/Game/Blueprints/UI/HUD/BP_HUD.BP_HUD_C|GetStatHUD _asbp_hud) true)
  (CallFunction|CreateNotificationPopup (Variables|/Game/Blueprints/UI/HUD/BP_HUD.BP_HUD_C|GetStatHUD _asbp_hud) " 
Put out the raging fire!  
" (Variables|Default|GetBurningHouseImage)))