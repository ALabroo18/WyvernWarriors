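; BP_Bounds is a level-bounds actor meant to show an animated out-of-bounds warning widget for the current island level.
; Re-entering BoundsTrigger clears OutOfBounds and removes the Level 2 widget.
; A DoOnce leads to a level-name switch that shows that level's widget, removes it after a delay and resets the gate.
; The end-overlap event is empty, leaving the player-tag check that enters the DoOnce disconnected.
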(event OnComponentEndOverlap(BoundsTrigger)
  (params (OverlappedComponent :type Primitive%20Component%20Object%20Reference) (OtherActor :type Actor%20Object%20Reference) (OtherComp :type Primitive%20Component%20Object%20Reference) (OtherBodyIndex :type Integer)))

(event OnComponentBeginOverlap(BoundsTrigger)
  (params (OverlappedComponent :type Primitive%20Component%20Object%20Reference) (OtherActor :type Actor%20Object%20Reference) (OtherComp :type Primitive%20Component%20Object%20Reference) (OtherBodyIndex :type Integer) (bFromSweep :type Boolean) (SweepResult :type Hit%20Result%20Structure%20%28by%20ref%29))
  (if (Variables|Default|GetoutOfBounds)
    (Variables|Default|SetoutOfBounds false)
    (bind _widget (Variables|Default|GetWidget)
      (:then
        (Widget|RemovefromParent _widget))
      (:else))))

(event Custom|CustomEvent)

(event Custom|resetsand
  (Utilities|FlowControl|DoOnce false) ; enters at Reset
)

(event EventBeginPlay)

(event Collision|EventActorBeginOverlap
  (params (OtherActor :type Actor%20Object%20Reference)))

(event EventTick
  (params (DeltaSeconds :type Float%20%28single-precision%29)))

(fn ConstructionScript)