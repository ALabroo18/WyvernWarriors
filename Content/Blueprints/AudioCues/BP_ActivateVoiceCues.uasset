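; BP_ActivateVoiceCues is a work-in-progress Blueprint for triggering voice cues, with only the outpost set wired up.
; ActivateOutpostCues calls three sub-graphs back to back, with no delay, each playing a temporary sound at AudioCenterPoint's relative location.
; Each sub-graph sets a Pass flag, but none gates playback.
; The fire and weapon cue events are empty, and leftover flag-setting nodes are disconnected.
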(event Custom|ActivateOutpostCues
  ;[1 0.2416 0 0.5] Construction zone
  ;;[1 0.8391 0] Play Outpost Audio 1
  (|PlayOutpostAudio1)
  ;;[1 0.8391 0] Play Outpost Audio 2
  (|PlayOutpostAudio2)
  ;;[1 0.8391 0] Play Outpost Audio 3
  (|PlayoutpostAudio3))

(event Custom|ActivateFireCues
  ;[1 0.2416 0 0.5] Construction zone
  ;;[1 0 0 0.5] In-progress
)

(event Custom|ActivateWeaponCues
  ;[1 0.2416 0 0.5] Construction zone
  ;;[1 0 0 0.5] In-progress
)

(fn ConstructionScript)