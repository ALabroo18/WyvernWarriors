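; Health pickup actor that plays a sound and restores a quarter of max health when the Bp_wyvern player overlaps its sphere.
; It fakes consumption by teleporting far below its start point, then returns after a 30-second delay guarded by a recently-healed flag.
; Heals that would exceed a hard-coded 100 just set health to 100, leaving the pickup in place.
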(event OnComponentBeginOverlap(Sphere)
  (params (OverlappedComponent :type Primitive%20Component%20Object%20Reference) (OtherActor :type Actor%20Object%20Reference) (OtherComp :type Primitive%20Component%20Object%20Reference) (OtherBodyIndex :type Integer) (bFromSweep :type Boolean) (SweepResult :type Hit%20Result%20Structure%20%28by%20ref%29))
  ;[0.15 0.15 0.15 0.5] Gives player 1/4th of their max health, moves to another location, and makes sure it doesn't heal twice.
  (bind _asbp_wyvern (Utilities|Casting|CastToBp_wyvern OtherActor))
  (bind _output_get (Variables|Default|SetPlayer _asbp_wyvern))
  (Audio|PlaySound2D "/Game/SFX/HealthPickup.HealthPickup" 0.2 1.0 0.0 0 0)
  (Variables|Default|SetCurrentHealth (+ (Variables|/Game/Blueprints/UI/HUD/BPA_CharacterStats.BPA_CharacterStats_C|GetHealth _output_get) (/ (Variables|/Game/Blueprints/UI/HUD/BPA_CharacterStats.BPA_CharacterStats_C|GetMaxHealth _output_get) 4.0)))
  (if (<= (+ (Variables|/Game/Blueprints/UI/HUD/BPA_CharacterStats.BPA_CharacterStats_C|GetHealth _output_get) (/ (Variables|/Game/Blueprints/UI/HUD/BPA_CharacterStats.BPA_CharacterStats_C|GetMaxHealth _output_get) 4.0)) 1e+02)
    (Variables|/Game/Blueprints/UI/HUD/BPA_CharacterStats.BPA_CharacterStats_C|SetHealth (Variables|Default|GetPlayer) (Variables|Default|GetCurrentHealth))
    (Transformation|Teleport (Variables|Default|GetSisterLocation) "0, 0, 0")
    (if (not (Variables|Default|GethasHealedRecently))
      (Variables|Default|SethasHealedRecently true)
      (Utilities|FlowControl|Delay 3e+01)
      (Transformation|Teleport (Variables|Default|GetInitialLocation) "0, 0, 0")
      (Variables|Default|SethasHealedRecently false))
    (else
      (Variables|/Game/Blueprints/UI/HUD/BPA_CharacterStats.BPA_CharacterStats_C|SetHealth (Variables|Default|GetPlayer) 1e+02))))

(event EventBeginPlay
  ;[0.15 0.15 0.15 0.5] Sets location for item to tp to in order to make it seem like the item was used
  (bind _output_get (Variables|Default|SetInitialLocation (Transformation|GetActorLocation)))
  (Variables|Default|SetSisterLocation (- _output_get "0.000000,0.000000,100000.000000"))
  (Variables|Default|SethasHealedRecently false))

(fn ConstructionScript)