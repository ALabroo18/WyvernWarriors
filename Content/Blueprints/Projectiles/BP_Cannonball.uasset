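; BP_Cannonball is a projectile the wyvern can pick up, used to destroy the boss's force field.
; A sphere overlap reports the wyvern entering or leaving range through the EventBus, hiding the pickup widget while in range and showing it again on exit.
; Once fired, a static mesh overlap with BP_Boss calls DestroyForceField, then resets the cannonball.
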(event OnComponentBeginOverlap(SphereComponent)
  (params (OverlappedComponent :type Primitive%20Component%20Object%20Reference) (OtherActor :type Actor%20Object%20Reference) (OtherComp :type Primitive%20Component%20Object%20Reference) (OtherBodyIndex :type Integer) (bFromSweep :type Boolean) (SweepResult :type Hit%20Result%20Structure%20%28by%20ref%29))
  ;[0.15 0.15 0.15 0.5] Call delegate when wyvern can/can't pickup cannonball
  (Utilities|IsValid OtherActor
    (:Is%20Valid
      (if (Class|GameplayStatics|ObjectIsA OtherActor "/Game/Blueprints/Characters/Wyvern/Bp_wyvern.Bp_wyvern_C")
        (Default|CallWyvernCanPickUpCannonball (Variables|Default|GetEventBus) true self)
        (Rendering|SetVisibility (Variables|Default|GetPickupWidget) false false)))))

(event OnComponentEndOverlap(SphereComponent)
  (params (OverlappedComponent :type Primitive%20Component%20Object%20Reference) (OtherActor :type Actor%20Object%20Reference) (OtherComp :type Primitive%20Component%20Object%20Reference) (OtherBodyIndex :type Integer))
  ;[0.15 0.15 0.15 0.5] Call delegate when wyvern can/can't pickup cannonball
  (Utilities|IsValid OtherActor
    (:Is%20Valid
      (if (Class|GameplayStatics|ObjectIsA OtherActor "/Game/Blueprints/Characters/Wyvern/Bp_wyvern.Bp_wyvern_C")
        (Default|CallWyvernCanPickUpCannonball (Variables|Default|GetEventBus) false self)
        (Rendering|SetVisibility (Variables|Default|GetPickupWidget) true false)))))

(event OnComponentBeginOverlap(StaticMesh)
  (params (OverlappedComponent :type Primitive%20Component%20Object%20Reference) (OtherActor :type Actor%20Object%20Reference) (OtherComp :type Primitive%20Component%20Object%20Reference) (OtherBodyIndex :type Integer) (bFromSweep :type Boolean) (SweepResult :type Hit%20Result%20Structure%20%28by%20ref%29))
  ;[0.15 0.15 0.15 0.5] Damage boss force field
  (if (Variables|Default|GetbHasBeenFired)
    (bind _asbp_boss (Utilities|Casting|CastToBP_Boss OtherActor))
    (Class|BossEnemy|DestroyForceField _asbp_boss)
    (Class|Cannonball|ResetCannonball)))

(event EventBeginPlay
  ;[0.15 0.15 0.15 0.5] Sets UI to on when spawned in
)

(fn ConstructionScript)