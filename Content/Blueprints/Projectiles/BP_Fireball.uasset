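; BP_Fireball is a homing projectile fired by the player's wyvern that damages enemies on contact.
; On BeginPlay it sets the targeted enemy's root as the projectile's homing target.
; Sphere overlaps ignore the wyvern; an EnemyBase hit takes damage amplified by the player's WyvernCombo component, with an explosion sound.
; Any overlap other than the wyvern, enemy or not, destroys the fireball.
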(event OnComponentBeginOverlap(Sphere)
  (params (OverlappedComponent :type Primitive%20Component%20Object%20Reference) (OtherActor :type Actor%20Object%20Reference) (OtherComp :type Primitive%20Component%20Object%20Reference) (OtherBodyIndex :type Integer) (bFromSweep :type Boolean) (SweepResult :type Hit%20Result%20Structure%20%28by%20ref%29))
  (CallFunction|FireballEnterOverlap OtherActor))

(event EventBeginPlay
  ;[0.15 0.15 0.15 0.5] Fireball Homing
  (Utilities|IsValid (Variables|Default|GetTargetedEnemy)
    (:Is%20Valid
      (Variables|/Script/Engine.ProjectileMovementComponent|SetHomingTargetComponent (Variables|Default|GetProjectileMovement) (Variables|/Script/Engine.Actor|GetRootComponent (Variables|Default|GetTargetedEnemy))))))

(fn ConstructionScript)

(fn FireballEnterOverlap
  (params (OverlappingActor :type Actor%20Object%20Reference))
  ;[0.15 0.15 0.15 0.5] Returns if overlapping player, else damages enemy if overlapped and destroys self
  (bind _output_get (LocalVariables|SetOverlappedActor OverlappingActor))
  (if (Class|GameplayStatics|ObjectIsA _output_get "/Game/Blueprints/Characters/Wyvern/Bp_wyvern.Bp_wyvern_C")
    (return)
    (else
      (if (Class|GameplayStatics|ObjectIsA (LocalVariables|GetOverlappedActor) "/Script/WyvernWarriors.EnemyBase")
        (bind _asbp_wyvern (Utilities|Casting|CastToBp_wyvern (Game|Player|GetPlayerPawn 0)))
        (bind _outdamage (Default|DoDamageAmp (Variables|/Game/Blueprints/Characters/Wyvern/Bp_wyvern.Bp_wyvern_C|GetWyvernCombo _asbp_wyvern) (Variables|Default|GetDamage)))
        (Game|Damage|ApplyDamage (LocalVariables|GetOverlappedActor) _outdamage 0 self)
        (Audio|SpawnSoundatLocation "/Game/SFX/FireballExplosion.FireballExplosion" (Transformation|GetActorLocation) "0, 0, 0" 1.0 1.0 0.0 "/Game/SFX/Fireball_Attenuation.Fireball_Attenuation" 0 false))
      (Actor|DestroyActor)
      (return))))