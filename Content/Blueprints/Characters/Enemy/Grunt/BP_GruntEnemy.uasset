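; Grunt enemy Blueprint with a health bar, awareness of nearby grunts and optional spline-only movement.
; A detection sphere maintains the array of nearby grunts, while damage lowers health and refreshes the bar, which turns toward the player each tick.
; Spline-only mode stops the AI brain and moves the grunt on a fast looping timer.
; Helper functions map fleeing, approaching and patrolling to speeds and add combo kills through the GameManager game instance.
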(event OnComponentBeginOverlap(DetectionSphere)
  (params (OverlappedComponent :type Primitive%20Component%20Object%20Reference) (OtherActor :type Actor%20Object%20Reference) (OtherComp :type Primitive%20Component%20Object%20Reference) (OtherBodyIndex :type Integer) (bFromSweep :type Boolean) (SweepResult :type Hit%20Result%20Structure%20%28by%20ref%29))
  ;[0.15 0.15 0.15 0.5] Add enemies to nearby enemies array
  (Utilities|IsValid OtherActor
    (:Is%20Valid
      (bind _asbp_grunt_enemy (Utilities|Casting|CastToBP_GruntEnemy OtherActor))
      (Utilities|Array|Add (Variables|Default|GetNearbyEnemies) _asbp_grunt_enemy))))

(event OnComponentEndOverlap(DetectionSphere)
  (params (OverlappedComponent :type Primitive%20Component%20Object%20Reference) (OtherActor :type Actor%20Object%20Reference) (OtherComp :type Primitive%20Component%20Object%20Reference) (OtherBodyIndex :type Integer))
  ;[0.15 0.15 0.15 0.5] Remove enemies from nearby enemies array
  (Utilities|IsValid OtherActor
    (:Is%20Valid
      (bind _asbp_grunt_enemy (Utilities|Casting|CastToBP_GruntEnemy OtherActor))
      (Utilities|Array|RemoveItem (Variables|Default|GetNearbyEnemies) _asbp_grunt_enemy))))

(event Custom|SplineMoverHelper
  ;[0.15 0.15 0.15 0.5] Makes Enemy Only Move Along Spline
  (Class|EnemyBase|MoveAlongSpline (Utilities|Time|GetWorldDeltaSeconds)))

(event EventSetHealthBarPercent
  (bind _healthbarwidget (Variables|Default|GetHealthBarWidget))
  ;[0.15 0.15 0.15 0.5] Set's fill for health bar
  (Utilities|IsValid _healthbarwidget
    (:Is%20Valid
      (bind _asenemy_ui (Utilities|Casting|CastToEnemyUI (UserInterface|GetUserWidgetObject _healthbarwidget)))
      (Progress|SetPercent (Variables|/Game/UI/EnemyStuff/EnemyUI.EnemyUI_C|GetEnemyHealth _asenemy_ui) (/ (Variables|Default|GetCurrentHealth) (Variables|Default|GetMaxHealth))))))

(event EventTick
  (params (DeltaSeconds :type Float%20%28single-precision%29))
  ;[0.15 0.15 0.15 0.5] Rotates health towards player
  (Class|GruntEnemy|TurnHealthBarTowardsPlayer))

(event Game|Damage|EventAnyDamage
  (params (Damage :type Float%20%28single-precision%29) (DamageType :type Damage%20Type%20Object%20Reference) (InstigatedBy :type Controller%20Object%20Reference) (DamageCauser :type Actor%20Object%20Reference))
  ;[0.15 0.15 0.15 0.5] Event for taking damage
  (Class|EnemyBase|ModifyCurrentHealth (* Damage -1.0))
  (Class|EnemyBase|SetHealthBarPercent))

(event EventMoveAlongSplineOnly
  ;[0.15 0.15 0.15 0.5] Makes Enemy Only Move Along Spline
  (AI|Logic|StopLogic (Variables|/Script/AIModule.AIController|GetBrainComponent (AI|GetAIController self)) "")
  (Utilities|Time|SetTimerbyEvent (delegate Custom|SplineMoverHelper) 0.01 true true))

(fn ConstructionScript)

(fn SetMovementSpeed
  (params (Speed :type MovementSpeedEnum%20Enum :default "NewEnumerator0"))
  (return (Utilities|Select :Index Speed :NewEnumerator0 3e+03 :NewEnumerator1 2.5e+03 :NewEnumerator2 2e+03)))

(fn IncreaseKillCombo
  (bind _asgame_manager (Utilities|Casting|CastToGameManager (Game|GetGameInstance)))
  (Default|AddComboKill _asgame_manager))