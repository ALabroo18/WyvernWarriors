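; Fireball projectile fired by the Grunt enemy, which homes toward the player and checks for a player to damage on overlap.
; Tick drives the homing and the sphere overlap triggers the damage check, both through functions defined outside these graphs.
; The construction script stores its projectile movement component in a variable.
; BeginPlay and EndPlay add and remove it from the GameManager game instance's enemy fireball count.
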(event OnComponentBeginOverlap(Sphere)
  (params (OverlappedComponent :type Primitive%20Component%20Object%20Reference) (OtherActor :type Actor%20Object%20Reference) (OtherComp :type Primitive%20Component%20Object%20Reference) (OtherBodyIndex :type Integer) (bFromSweep :type Boolean) (SweepResult :type Hit%20Result%20Structure%20%28by%20ref%29))
  (Class|GruntEnemyProjectile|CheckforPlayertoDamage OtherActor))

(event EventBeginPlay
  ;[0.15 0.15 0.15 0.5] Add/Remove Fireball Count in Game Manager
  (bind _asgame_manager (Utilities|Casting|CastToGameManager (Game|GetGameInstance)))
  (bind _output_get (Variables|Default|SetAs%20Game%20Manager _asgame_manager))
  (Default|AddEnemyFireball _output_get))

(event EventEndPlay
  (params (EndPlayReason :type EEndPlayReason%20Enum :default "Destroyed"))
  ;[0.15 0.15 0.15 0.5] Add/Remove Fireball Count in Game Manager
  (Default|RemoveEnemyFireball (Variables|Default|GetAs%20Game%20Manager)))

(event EventTick
  (params (DeltaSeconds :type Float%20%28single-precision%29))
  (Class|GruntEnemyProjectile|HomeTowardsPlayer))

(fn ConstructionScript
  (Variables|Default|SetProjectileMovementComponent (Variables|Default|GetProjectileMovement)))