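; Boss enemy character that fights the player's wyvern and can trigger a final-blow quick time event.
; Mesh hits apply collision damage to the wyvern.
; Incoming damage lowers health through ModifyCurrentHealth only while the forcefield is inactive.
; PlayFinalBlowQTE creates the boss QTE widget for the first player controller and calls its setup.
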(event OnComponentHit(SkeletalMesh)
  (params (HitComponent :type Primitive%20Component%20Object%20Reference) (OtherActor :type Actor%20Object%20Reference) (OtherComp :type Primitive%20Component%20Object%20Reference) (NormalImpulse :type Vector :default "0, 0, 0") (Hit :type Hit%20Result%20Structure%20%28by%20ref%29))
  ;[0.15 0.15 0.15 0.5] Collision Damage for Player
  (bind _asbp_wyvern (Utilities|Casting|CastToBp_wyvern OtherActor))
  (Game|Damage|ApplyDamage _asbp_wyvern (Variables|Default|GetCollisionDamageAmount) 0 self))

(event Game|Damage|EventAnyDamage
  (params (Damage :type Float%20%28single-precision%29) (DamageType :type Damage%20Type%20Object%20Reference) (InstigatedBy :type Controller%20Object%20Reference) (DamageCauser :type Actor%20Object%20Reference))
  ;[0.15 0.15 0.15 0.5] Take damage if no forcefield
  (if (not (Variables|Default|GetbIsForcefieldActive))
    (Class|EnemyBase|ModifyCurrentHealth (* Damage -1.0))))

(event EventPlayFinalBlowQTE
  (bind _asboss_qtewidget (Utilities|Casting|CastToBoss_QTEWidgetClass (Variables|Default|GetFinalBlowQTE)))
  (bind _returnvalue (UserInterface|CreateWidget _asboss_qtewidget (Game|GetPlayerController 0)))
  (Default|SetupBossQTE _returnvalue))

(fn ConstructionScript)