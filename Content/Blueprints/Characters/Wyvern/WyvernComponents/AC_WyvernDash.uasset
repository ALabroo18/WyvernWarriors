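; Wyvern actor component that provides a stamina-limited dash.
; DashSetVelocity overrides the owner's CharacterMovement velocity along its forward vector and drains one point of StaminaMeter on the player's WyvernControl per call.
; At zero stamina it calls TurnOffDash on the controller and starts a looping timer on ResetStamina, which adds stamina in steps with no clamp or stop in this component.
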(event EventBeginPlay
  (Utilities|Casting|CastToBp_wyvern (Variables|Default|Getbp_wyvernRef))
  (Variables|Default|Setbp_wyvernRef 0)
  (bind _aswyvern_control (Utilities|Casting|CastToWyvernControl (Game|GetPlayerController 0)))
  (Variables|Default|SetwyverncontrolRef _aswyvern_control))

(fn DashSetVelocity
  (bind _returnvalue (Components|GetOwner))
  (bind _returnvalue_2 (Actor|GetComponentbyClass _returnvalue "/Script/Engine.CharacterMovementComponent"))
  (Utilities|IsValid _returnvalue_2
    (:Is%20Valid
      (if true
        (Variables|/Script/Engine.MovementComponent|SetVelocity _returnvalue_2 (* (Transformation|GetActorForwardVector _returnvalue) "10000.000000,10000.000000,10000.000000"))
        (bind _aswyvern_control (Utilities|Casting|CastToWyvernControl (Game|GetPlayerController 0)))
        (Variables|Default|SetwyverncontrolRef _aswyvern_control)
        (Utilities|IsValid (Variables|Default|GetwyverncontrolRef)
          (:Is%20Valid
            (bind _result (Math|Integer|DecrementInt (Variables|/Game/Blueprints/WyvernControl.WyvernControl_C|GetStaminaMeter (Variables|Default|GetwyverncontrolRef)))
              (:%20%20
                (if (<= (Variables|/Game/Blueprints/WyvernControl.WyvernControl_C|GetStaminaMeter (Variables|Default|GetwyverncontrolRef)) 0)
                  (Default|TurnOffDash (Variables|Default|GetwyverncontrolRef))
                  (Development|PrintString (Utilities|String|ToString(Integer) _result) true true "(R=0.000000,G=0.660000,B=1.000000,A=1.000000)" 0.0)
                  (Utilities|Time|SetTimerbyFunctionName 0 "ResetStamina" 3.0 true))))))))))

(fn ResetStamina
  (Variables|/Game/Blueprints/WyvernControl.WyvernControl_C|SetStaminaMeter (Variables|Default|GetwyverncontrolRef) (+ (Variables|/Game/Blueprints/WyvernControl.WyvernControl_C|GetStaminaMeter (Variables|Default|GetwyverncontrolRef)) 10)))