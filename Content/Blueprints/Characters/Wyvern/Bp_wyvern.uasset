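; Player-controlled wyvern with constant-forward flight, combat skills, pause menu and wave-based save/load.
; Tick sweeps it forward with speed adjusted by pitch, while dive and hover logic interpolate speed, dive also widening camera FOV.
; Sphere traces drive enemy lock-on, which steers rotation and targets fireballs, and a melee dash at weakened grunts.
; Flamethrower unlocks on the final wave, timers spawn limited water, and hard terrain hits bounce and stun.
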(event OnComponentHit(Mesh)
  (params (HitComponent :type Primitive%20Component%20Object%20Reference) (OtherActor :type Actor%20Object%20Reference) (OtherComp :type Primitive%20Component%20Object%20Reference) (NormalImpulse :type Vector :default "0, 0, 0") (Hit :type Hit%20Result%20Structure%20%28by%20ref%29))
  (Utilities|IsValid OtherActor
    (:Is%20Valid
      (if (Actor|ActorHasTag OtherActor "Meter.Enemy")
        (Game|Damage|ApplyDamage self 25.0 0 0)))))

(event OnComponentEndOverlap(FlameDamage)
  (params (OverlappedComponent :type Primitive%20Component%20Object%20Reference) (OtherActor :type Actor%20Object%20Reference) (OtherComp :type Primitive%20Component%20Object%20Reference) (OtherBodyIndex :type Integer))
  ;[0.15 0.15 0.15 0.5] For Flamethrower
)

(event OnComponentHit(CapsuleComponent)
  (params (HitComponent :type Primitive%20Component%20Object%20Reference) (OtherActor :type Actor%20Object%20Reference) (OtherComp :type Primitive%20Component%20Object%20Reference) (NormalImpulse :type Vector :default "0, 0, 0") (Hit :type Hit%20Result%20Structure%20%28by%20ref%29))
  (if (Variables|Default|GetisUsingMelee)
    (bind _asbp_grunt_enemy (Utilities|Casting|CastToBP_GruntEnemy OtherActor))
    (Game|Damage|ApplyDamage _asbp_grunt_enemy 2e+02 0 self)
    (else
      (Variables|Default|SetActualMaxSpeed 3e+02))))

(event OnComponentBeginOverlap(FlameThrowerDamage)
  (params (OverlappedComponent :type Primitive%20Component%20Object%20Reference) (OtherActor :type Actor%20Object%20Reference) (OtherComp :type Primitive%20Component%20Object%20Reference) (OtherBodyIndex :type Integer) (bFromSweep :type Boolean) (SweepResult :type Hit%20Result%20Structure%20%28by%20ref%29))
  ;[0.15 0.15 0.15 0.5] For Flamethrower
  (bind _asenemy_base (Utilities|Casting|CastToEnemyBase OtherActor))
  (Utilities|Time|SetTimerbyFunctionName 0 "SprayDamageTick" 0.5 true true)
  (Game|Damage|ApplyDamage _asenemy_base 45.0 0 self))

(event Custom|SpawnPlayer
  ;[0.15 0.15 0.15 0.5] Spawn Wyvern in Game
  (bind _asbp_wyvern (Utilities|Casting|CastToBp_wyvern (Game|GetPlayerCharacter 0)))
  (bind _output_get (Variables|Default|SetActiveChar _asbp_wyvern))
  (CallFunction|UpdateUI _output_get))

(event Custom|ClearHasWeapon
  ;[0.15 0.15 0.15 0.5] WeaponQTE (WIP)
  (Variables|Default|SetHasWeapon false))

(event Custom|Hover
  ;[0.15 0.15 0.15 0.5] S To Slow Down
  (bind _aswyvern_control (Utilities|Casting|CastToWyvernControl (Pawn|GetController)))
  (if (not (Variables|/Game/Blueprints/WyvernControl.WyvernControl_C|GetbisDoingAction _aswyvern_control))
    (if (Variables|Default|GetisSlowingDown)
      (bind _output_get (Variables|Default|SetActualMaxSpeed (Math|Interpolation|FInterptoConstant (Variables|Default|GetActualMaxSpeed) (Variables|Default|GetHoverState) 0.2 2e+02)))
      (Development|PrintString (Utilities|String|ToString(Float) (Variables|Default|GetActualMaxSpeed)))
      (if (<= _output_get 5e+02)
        (Variables|Default|SetisHovering true)
        (Animation|Montage|PlayMontage (Variables|Character|GetMesh) "/Game/Animations/Dragon_Hover_Anim_Montage.Dragon_Hover_Anim_Montage"))
      (elif (>= (Variables|Default|GetActualMaxSpeed) 2e+03)
        (Variables|Default|SetisHovering false)
        (Animation|Montage|MontageStop (Components|SkeletalMesh|GetAnimInstance (Variables|Character|GetMesh)) 0.5 "/Game/Animations/Dragon_Hover_Anim_Montage.Dragon_Hover_Anim_Montage")))))

(event Custom|DiveState
  ;[0.15 0.15 0.15 0.5] Speed Momentum/Smooth Out
  (if (and (not (Variables|Default|GetisSlowingDown)) (not (Variables|Default|GetbCameraOverride)))
    (if (<= (CallFunction|GetPitch) 5e+01)
      (Variables|Default|SetActualMaxSpeed (Math|Interpolation|FInterpTo (Variables|Default|GetActualMaxSpeed) (Variables|Default|GetMaxDiveSpeed) (Utilities|Time|GetWorldDeltaSeconds) 0.2))
      (Camera|SetFieldOfView (Variables|Default|GetCamera) (Math|Interpolation|FInterpTo (Variables|/Script/Engine.CameraComponent|GetFieldOfView (Variables|Default|GetCamera)) 1.3e+02 (Utilities|Time|GetWorldDeltaSeconds) 0.5))
      (if (>= (Variables|Default|GetActualMaxSpeed) 8e+03)
        (Game|Feedback|ClientStartCameraShake (Game|GetPlayerController 0) "/Game/Blueprints/Bp_dashCameraShake.Bp_dashCameraShake_C" 1.0 "CameraLocal" "0, 0, 0")
        (Development|PrintString (Utilities|String|ToString(Float) (Variables|Default|GetActualMaxSpeed)) true true "(R=1.000000,G=0.001108,B=0.000000,A=1.000000)"))
      (else
        (Variables|Default|SetActualMaxSpeed (Math|Interpolation|FInterpTo (Variables|Default|GetActualMaxSpeed) 3e+03 (Utilities|Time|GetWorldDeltaSeconds) 0.5))
        (Camera|SetFieldOfView (Variables|Default|GetCamera) (Math|Interpolation|FInterpTo (Variables|/Script/Engine.CameraComponent|GetFieldOfView (Variables|Default|GetCamera)) 9e+01 (Utilities|Time|GetWorldDeltaSeconds) 1.0))))))

(event Custom|ShowQTE
  (params (PromptText :type Text%20%28by%20ref%29))
  ;[0.15 0.15 0.15 0.5] WeaponQTE (WIP)
  (bind _returnvalue (UserInterface|CreateWidget "/Game/Blueprints/UI/HUD/WBP_InteractionPrompt.WBP_InteractionPrompt_C"))
  (bind _output_get (Variables|Default|SetInteractionWidget _returnvalue))
  (UserInterface|Viewport|AddtoViewport _output_get 0)
  (Widget|SetVisibility (Variables|Default|GetInteractionWidget) "Visible"))

(event Custom|HideQTE
  ;[0.15 0.15 0.15 0.5] WeaponQTE (WIP)
  (Widget|SetVisibility (Variables|Default|GetInteractionWidget) "Hidden"))

(event Custom|MeleeInteract
  ;[0.15 0.15 0.15 0.5] Melee
  (Variables|Default|SetisUsingMelee false))

(event Custom|SprayDamageTick
  ;[0.15 0.15 0.15 0.5] For Flamethrower
  (Utilities|Time|SetTimerbyFunctionName 0 "SprayDamageTick" 0.5 true true)
  (Game|Damage|ApplyDamage (stale OnComponentBeginOverlap(FlameThrowerDamage) _asenemy_base) 45.0 0 self))

(event Custom|SpawnWaterEvent
  ;[0.15 0.15 0.15 0.5] How the Player Spawns Water
  (if (Variables|WaterQTE|GetShootingWater)
    (bind _returnvalue (Utilities|Time|SetTimerbyFunctionName 0 "SpawnWater" (Variables|WaterQTE|GetWaterSpawnTimer) true true))
    (Variables|WaterQTE|SetSpawnWaterFunction _returnvalue)
    (else
      (Utilities|Time|ClearandInvalidateTimerbyHandle (Variables|WaterQTE|GetSpawnWaterFunction)))))

(event Custom|NewWaveEvent
  (params (BIsFinalWave :type Boolean))
  ;[0.15 0.15 0.15 0.5] 360 movement
  (if BIsFinalWave
    (Variables|Default|SetbFlamethrowerUnlocked true)
    (bind _returnvalue (UserInterface|CreateWidget "/Game/UI/Wb_FlamethrowerPickup.Wb_FlamethrowerPickup_C"))
    (Variables|/Game/UI/Wb_FlamethrowerPickup.Wb_FlamethrowerPickup_C|SetPickupMessage _returnvalue "Flamethrower Unlocked!")
    (UserInterface|Viewport|AddtoViewport _returnvalue 0)))

(event Custom|EndStun
  ;[0.15 0.15 0.15 0.5] Terrain Collision
  (Variables|/Game/Blueprints/WyvernControl.WyvernControl_C|SetbisDoingAction (stale Collision|EventHit _aswyvern_control) false)
  (Variables|Default|SetYawSpeed 0.3))

(event Collision|EventHit
  (params (MyComp :type Primitive%20Component%20Object%20Reference) (Other :type Actor%20Object%20Reference) (OtherComp :type Primitive%20Component%20Object%20Reference) (bSelfMoved :type Boolean) (HitLocation :type Vector :default "0, 0, 0") (HitNormal :type Vector :default "0, 0, 0") (NormalImpulse :type Vector :default "0, 0, 0") (Hit :type Hit%20Result%20Structure%20%28by%20ref%29))
  ;[0.15 0.15 0.15 0.5] Terrain Collision
  (Utilities|Casting|CastToBp_wyvern Other
    (:CastFailed
      (Variables|/Script/Engine.MovementComponent|SetVelocity (Variables|Default|GetFloatingPawnMovement) (* HitNormal 5e+03))
      (if (and (>= (Variables|Default|GetActualMaxSpeed) 4e+03) (not (Actor|ActorHasTag Other "Meter.Enemy")))
        (bind _aswyvern_control (Utilities|Casting|CastToWyvernControl (Pawn|GetController)))
        (Variables|/Game/Blueprints/WyvernControl.WyvernControl_C|SetbisDoingAction _aswyvern_control true)
        (Variables|Default|SetYawSpeed 0.1)
        (Animation|Montage|PlayMontage (Variables|Character|GetMesh) "/Game/Animations/Hurt_Montage.Hurt_Montage"
          (:OnCompleted
            _)
          (:OnInterrupted
            _))
        (Utilities|Time|SetTimerbyEvent (delegate Custom|EndStun) 1.0 false true)))))

(event EventTick
  (params (DeltaSeconds :type Float%20%28single-precision%29))
  (Utilities|FlowControl|Sequence
    (:then_0
      (Variables|Default|GetLockedOnEnemy
        (:then
          (Pawn|SetControlRotation (Pawn|GetController) (Math|Interpolation|RInterpTo (Transformation|GetActorRotation) (Math|Rotator|FindLookatRotation (Transformation|GetActorLocation) (Transformation|GetActorLocation (Variables|Default|GetLockedOnEnemy))) (Utilities|Time|GetWorldDeltaSeconds) 5.0)))
        (:else)))
    (:then_1
      (Utilities|MovePlayerForward DeltaSeconds
        (:End
          (Utilities|FlowControl|Delay 0.2)
          (CallFunction|SpawnPlayer))))))

(event EventBeginPlay
  ;[0.15 0.15 0.15 0.5] 360 movement
  (Utilities|FlowControl|Sequence
    (:then_0
      (bind _asgame_manager (Utilities|Casting|CastToGameManager (Game|GetGameInstance)))
      (Variables|Default|SetAs%20Game%20Manager _asgame_manager))
    (:then_1
      (bind _wave_management_component (CallFunction|GetWaveManagementComponent))
      (bind _output_get (Variables|Default|SetWave%20Management%20Component _wave_management_component))
      (EventDispatchers|BindEventtoOnNewWave _output_get (delegate Custom|NewWaveEvent))
      (bind _game_state_level (CallFunction|GetGameStateLevel))
      (Variables|Default|SetGame%20State%20Level _game_state_level)
      (bind _enemymanagementcomponent (CallFunction|GetEnemyManagementComponent))
      (Variables|Default|SetEnemy%20Management%20Component _enemymanagementcomponent))
    (:then_2
      ;[0.15 0.15 0.15 0.5] Set Water QTE Visibility, Material, and Controller Sensitivity
      (CallFunction|SetWyvernMaterial)
      (CallFunction|SetControlSensitivity)
      (Rendering|SetVisibility (Variables|Default|GetWaterQTEIcon) true false))
    (:then_3
      ;[0.15 0.15 0.15 0.5] Set Control Sensitivity
      (bind _asgame_manager_2 (Utilities|Casting|CastToGameManager (Game|GetGameInstance)))
      (Default|UpdateSensitivity _asgame_manager_2)
      (CallFunction|ChooseInputType))
    (:then_4
      ;[0.15 0.15 0.15 0.5] Set Tutorial Manager Instance
      (bind _returnvalue (Actor|GetActorOfClass "/Game/Blueprints/Tutorial/BP_TutorialManager.BP_TutorialManager_C"))
      (Variables|Default|SetTutorialManagerInst _returnvalue))
    (:then_5
      (CallFunction|InitializeDiveStateTimers))
    (:then_6
      (CallFunction|InitializeHovering))
    (:then_7
      (CallFunction|MovementonStart))
    (:then_8
      ;[0.15 0.15 0.15 0.5] Saves game to ensure save point for player to return to
      (CallFunction|SaveGame))))

(event Input|ActionEvents|InputActionPause
  (params (Key :type Key%20Structure :default "None"))
  (bind _returnvalue (Game|GetPlayerController 0))
  ;[0.15 0.15 0.15 0.5] PauseMenu
  (:Pressed
    (if (not (Variables|Default|GetisPausedMenuOpen))
      (Variables|Default|SetisPausedMenuOpen true)
      (bind _returnvalue_2 (UserInterface|CreateWidget "/Game/Blueprints/UI/MenuScreen/WB_PauseMenu.WB_PauseMenu_C" _returnvalue))
      (bind _output_get (Variables|Default|SetPaused%20Menu%20WIdget _returnvalue_2))
      (UserInterface|Viewport|AddtoViewport _output_get 0)
      (Input|SetInputModeGameandUI _returnvalue (Variables|Default|GetPaused%20Menu%20WIdget) "DoNotLock" true false)
      (Variables|/Script/Engine.PlayerController|SetbShowMouseCursor (Game|GetPlayerController 0) true)
      (Game|SetGamePaused true)
      (else
        (Variables|Default|SetisPausedMenuOpen false)
        (Widget|RemovefromParent (Variables|Default|GetPaused%20Menu%20WIdget))
        (Game|SetGamePaused false)
        (Input|SetInputModeGameOnly _returnvalue false)
        (Variables|/Script/Engine.PlayerController|SetbShowMouseCursor (Game|GetPlayerController 0) false)))))

(event Input|ActionEvents|InputActionSlowDown
  (params (Key :type Key%20Structure :default "None"))
  ;[0.15 0.15 0.15 0.5] S To Slow Down
  (:Pressed
    (Variables|Default|SetisSlowingDown true))
  (:Released
    (Variables|Default|SetisSlowingDown false)))

(event Input|ActionEvents|InputActionDashTackle
  (params (Key :type Key%20Structure :default "None"))
  (bind _returnvalue (Transformation|GetActorLocation))
  (bind _tutorialmanagerinst (Variables|Default|GetTutorialManagerInst))
  ;[0.15 0.15 0.15 0.5] Melee
  (:Pressed
    (bind _aswyvern_control (Utilities|Casting|CastToWyvernControl (Game|GetPlayerController 0)))
    (Default|InputDetection _aswyvern_control)
    (if true
      (bind _outhit (Collision|SphereTraceByChannel _returnvalue (+ (* (Transformation|GetActorForwardVector) 5e+03) _returnvalue) 5e+01 "TraceTypeQuery1" false 0 "None"))
      (bind _asbp_grunt_enemy (Utilities|Casting|CastToBP_GruntEnemy (.HitActor (Collision|BreakHitResult _outhit))))
      (Utilities|IsValid _asbp_grunt_enemy
        (:Is%20Valid
          (if (<= (/ (Variables|/Script/WyvernWarriors.EnemyBase|GetCurrentHealth _asbp_grunt_enemy) 2.0) 5e+01)
            (Physics|AddImpulse (Variables|Character|GetCharacterMovement) (* (Math|Vector|Normalize (- (Transformation|GetActorLocation (.HitActor (Collision|BreakHitResult _outhit))) (Transformation|GetActorLocation self))) 2e+04) true)
            (Game|Feedback|ClientStartCameraShake (Game|GetPlayerController 0) "/Game/Blueprints/Bp_dashCameraShake.Bp_dashCameraShake_C" 1.0 "CameraLocal" "0, 0, 0")
            (Variables|Default|SetisUsingMelee true)
            (Utilities|Time|SetTimerbyEvent (delegate Custom|MeleeInteract) 0.3)
            (Utilities|IsValid _tutorialmanagerinst
              (:Is%20Valid
                (Variables|/Game/Blueprints/Tutorial/BP_TutorialManager.BP_TutorialManager_C|SetbPlayerDidMelee _tutorialmanagerinst true) ; Tutorial Variable
              ))))))))

(event Input|ActionEvents|InputActionLockOn/GAMEPAD
  (params (Key :type Key%20Structure :default "None"))
  (bind _returnvalue (Transformation|GetActorLocation))
  ;[0.15 0.15 0.15 0.5] Hold Q to auto lock-on target, Release to let go. (In Progress)
  (:Pressed
    (bind _aswyvern_control (Utilities|Casting|CastToWyvernControl (Game|GetPlayerController 0)))
    (Default|InputDetection _aswyvern_control)
    (Utilities|FlowControl|FlipFlop
      (:A
        (bind (_outhit _returnvalue_2) (Collision|SphereTraceForObjects _returnvalue (+ _returnvalue (* (Math|Vector|GetForwardVector (Transformation|GetWorldRotation (Variables|Default|GetCamera))) 5e+02)) 1e+04 (Utilities|Array|MakeArray "ObjectTypeQuery3") false 0 "None"))
        (if _returnvalue_2
          (if (>= (Math|Vector|DotProduct (Math|Vector|Normalize (- (Transformation|GetActorLocation (.HitActor (Collision|BreakHitResult _outhit))) (Transformation|GetActorLocation self))) (Transformation|GetActorForwardVector)) 0.5)
            (bind _asbp_grunt_enemy (Utilities|Casting|CastToBP_GruntEnemy (.HitActor (Collision|BreakHitResult _outhit))))
            (bind _output_get (Variables|Default|SetLockedOnEnemy _asbp_grunt_enemy))
            (Class|GruntEnemy|HighlightGruntEnemy _output_get true))))
      (:B
        (Utilities|IsValid (Variables|Default|GetLockedOnEnemy)
          (:Is%20Valid
            (Class|GruntEnemy|HighlightGruntEnemy (Variables|Default|GetLockedOnEnemy) true))
          (:Is%20Not%20Valid
            _))
        (Variables|Default|SetLockedOnEnemy 0)))))

(event Input|AxisEvents|InputAxisMoveLeft/Right
  (params (AxisValue :type Float%20%28single-precision%29))
  (bind _returnvalue (Utilities|Time|GetWorldDeltaSeconds))
  (bind _returnvalue_2 (* AxisValue _returnvalue))
  ;[0.15 0.15 0.15 0.5] Moving up and down/speed
  (bind _aswyvern_control (Utilities|Casting|CastToWyvernControl (Game|GetPlayerController 0)))
  (Default|InputDetection _aswyvern_control)
  (Pawn|Input|AddControllerYawInput (* _returnvalue_2 (Variables|Default|GetYawSpeed) (Variables|Default|GetactiveSensitivity)))
  (bind _output_get (Variables|Transformation|SetCurrentPosition (Math|Float|Clamp(Float) (Math|Float|Lerp (Variables|Transformation|GetCurrentPosition) (* _returnvalue_2 (Variables|Default|GetmaxRollAngle)) (* (Utilities|Time|GetWorldDeltaSeconds) (Variables|Default|GetRollSpeed))) -2e+01 2e+01)))
  (Transformation|SetRelativeRotation (Variables|Character|GetMesh) (Math|Rotator|MakeRotator 0.0 _output_get 2.7e+02) true true))

(event Input|AxisEvents|InputAxisMoveUp/Down
  (params (AxisValue :type Float%20%28single-precision%29))
  ;[0.15 0.15 0.15 0.5] Moving up and down/speed
  (bind _aswyvern_control (Utilities|Casting|CastToWyvernControl (Game|GetPlayerController 0)))
  (Default|InputDetection _aswyvern_control)
  (Pawn|Input|AddControllerPitchInput (* (* AxisValue (Utilities|Time|GetWorldDeltaSeconds)) (Variables|Default|GetPitchSpeed) (Variables|Default|GetactiveSensitivity))))

(event Input|AxisEvents|InputAxisMoveUp/Down
  (params (AxisValue :type Float%20%28single-precision%29))
  ;[0.15 0.15 0.15 0.5] Moving up and down/speed
  (bind _aswyvern_control (Utilities|Casting|CastToWyvernControl (Game|GetPlayerController 0)))
  (Default|InputDetection _aswyvern_control)
  (Transformation|AddActorLocalOffset (Math|Vector|MakeVector 0.0 0.0 (* AxisValue 0.0)) false false)
  (Transformation|AddActorLocalRotation "0, 0, 0" false false))

(event Input|KeyboardEvents|Q
  (params (Key :type Key%20Structure :default "None"))
  (bind _returnvalue (Transformation|GetActorLocation))
  ;[0.15 0.15 0.15 0.5] Hold Q to auto lock-on target, Release to let go. (In Progress)
  (:Pressed
    (bind _aswyvern_control (Utilities|Casting|CastToWyvernControl (Game|GetPlayerController 0)))
    (Default|InputDetection _aswyvern_control)
    (Utilities|FlowControl|FlipFlop
      (:A
        (bind (_outhit _returnvalue_2) (Collision|SphereTraceForObjects _returnvalue (+ _returnvalue (* (Math|Vector|GetForwardVector (Transformation|GetWorldRotation (Variables|Default|GetCamera))) 5e+02)) 1e+04 (Utilities|Array|MakeArray "ObjectTypeQuery3") false 0 "None"))
        (if _returnvalue_2
          (if (>= (Math|Vector|DotProduct (Math|Vector|Normalize (- (Transformation|GetActorLocation (.HitActor (Collision|BreakHitResult _outhit))) (Transformation|GetActorLocation self))) (Transformation|GetActorForwardVector)) 0.5)
            (bind _asbp_grunt_enemy (Utilities|Casting|CastToBP_GruntEnemy (.HitActor (Collision|BreakHitResult _outhit))))
            (bind _output_get (Variables|Default|SetLockedOnEnemy _asbp_grunt_enemy))
            (Class|GruntEnemy|HighlightGruntEnemy _output_get true))))
      (:B
        (Utilities|IsValid (Variables|Default|GetLockedOnEnemy)
          (:Is%20Valid
            (Class|GruntEnemy|HighlightGruntEnemy (Variables|Default|GetLockedOnEnemy) true))
          (:Is%20Not%20Valid
            _))
        (Variables|Default|SetLockedOnEnemy 0)))))

(event Input|KeyboardEvents|O
  (params (Key :type Key%20Structure :default "None"))
  ;[0.15 0.15 0.15 0.5] Save and Load testing
  (:Pressed
    (CallFunction|SaveGame)))

(event Input|KeyboardEvents|L
  (params (Key :type Key%20Structure :default "None"))
  ;[0.15 0.15 0.15 0.5] Save and Load testing
  (:Pressed
    (CallFunction|LoadGame)))

(fn ConstructionScript)

(fn Damage)

(fn RegainMaxSpeed
  (if (< (Variables|Default|GetActualMaxSpeed) 3e+03)
    (bind _output_get (Variables|Default|SetActualMaxSpeed (+ (Variables|Default|GetActualMaxSpeed) (/ (Variables|Default|GetActualMaxSpeed) 5e+01))))
    (if (> _output_get 3e+02)
      (Variables|Default|SetActualMaxSpeed 3e+03 :!label _label))
    (else
      (goto _label))))

(fn Fireball
  (if (Variables|Default|GetisReady)
    (Game|SpawnActorfromClass "/Game/Blueprints/Projectiles/BP_Fireball.BP_Fireball_C" (Transformation|GetWorldTransform (Variables|Default|GetSpawnPoint)) "Undefined" "MultiplyWithRoot" 0 (Variables|Default|GetLockedOnEnemy) 0)))

(fn FlamethrowerSkill
  (Utilities|FlowControl|Sequence
    (:then_0
      (if (Variables|Default|GetbFlamethrowerUnlocked)
        (Collision|SetCollisionEnabled (Variables|Default|GetFlameThrowerDamage) "QueryOnly")
        (Development|PrintString "overlapping")
        (Components|Activation|Activate (Variables|Default|GetFlamethrowerEffect) false)
        (Variables|Default|SetbFlamethrowerUnlocked false)
        (Components|Activation|Deactivate (Variables|Default|GetFlamethrowerEffect))
        (Variables|Default|SetbFlamethrowerUnlocked true)
        (else
          (Components|Activation|Deactivate (Variables|Default|GetFlamethrowerEffect) :!label _label))))
    (:then_1
      (Collision|SetCollisionEnabled (Variables|Default|GetFlameThrowerDamage) "NoCollision")
      (goto _label))))

(fn DashSkill
  (bind _returnvalue (Transformation|GetActorForwardVector))
  (bind _returnvalue_2 (* _returnvalue 1.5e+04))
  (if (Variables|Default|GetisAction)
    (Variables|Default|SetisAction true)
    (Variables|/Script/Engine.MovementComponent|SetVelocity (Variables|Character|GetCharacterMovement) (Math|Vector|MakeVector (.x _returnvalue_2) (.y _returnvalue_2) (.z _returnvalue_2)))))

(fn StartWaterQTE
  (Variables|WaterQTE|SetInWater true))

(fn SpawnWater
  ;[0.15 0.15 0.15 0.5] Spawns in water every WaterSpawnTimer seconds, and stops the event when playing stops shooting water
  (if (Variables|WaterQTE|GetShootingWater)
    (Game|SpawnActorfromClass "/Game/Blueprints/WaterQTE/Water.Water_C" (Transformation|GetWorldTransform (Variables|Default|GetWaterSpawnPoint)) "Undefined" "MultiplyWithRoot" 0 self)
    ;[0.15 0.15 0.15 0.5] Lowers the water remaining percentage for HUD, stops allowing water to be used when the water is out
    (bind _output_get (Variables|WaterQTE|SetWaterTimerRemaining (- (Variables|WaterQTE|GetWaterTimerRemaining) (Variables|WaterQTE|GetWaterSpawnTimer))))
    (if (<= _output_get 0.0)
      (Utilities|Time|ClearandInvalidateTimerbyHandle (Variables|WaterQTE|GetSpawnWaterFunction))
      (CallFunction|WaterOff))
    (else
      (Utilities|Time|ClearandInvalidateTimerbyHandle (Variables|WaterQTE|GetSpawnWaterFunction)))))

(fn WaterOff
  (Variables|WaterQTE|SetHasWater false)
  (Rendering|SetVisibility (Variables|Default|GetWaterQTEIcon) false false))

(fn SaveGame
  (Development|PrintString "Autosaving, please do not close the game at this time")
  (Utilities|FlowControl|Sequence
    (:then_0
      ;[0.15 0.15 0.15 0.5] Makes sure save reference exists, if not makes the reference
      (Utilities|IsValid (Variables|Saving|GetSave%20Game%20Ref)
        (:Is%20Not%20Valid
          (bind _returnvalue (SaveGame|CreateSaveGameObject "/Game/Blueprints/Saving/SaveGame.SaveGame_C"))
          (Variables|Saving|SetSave%20Game%20Ref _returnvalue))))
    (:then_1
      ;[0.15 0.15 0.15 0.5] Sequence 1 is all things to be saved
      (Utilities|FlowControl|Sequence
        (:then_0
          (Utilities|IsValid (Variables|Default|GetWave%20Management%20Component)
            (:Is%20Valid
              (Variables|/Game/Blueprints/Saving/SaveGame.SaveGame_C|SetNumOfWaves (Variables|Saving|GetSave%20Game%20Ref) (Class|GameStateLevel|GetCurrentWaveNumber (Variables|Default|GetGame%20State%20Level))))))
        (:then_1
          (Variables|/Game/Blueprints/Saving/SaveGame.SaveGame_C|SetHasFlamethrower (Variables|Saving|GetSave%20Game%20Ref) (Variables|Default|GetbFlamethrowerUnlocked)))))
    (:then_2
      ;[0.15 0.15 0.15 0.5] Saves game to slot
      (SaveGame|SaveGametoSlot (Variables|Saving|GetSave%20Game%20Ref) (Variables|Saving|GetSaveGameSlotFinalWave))
      (Development|PrintString "Game has been saved."))))

(fn LoadGame
  (bind _savegameslotfinalwave (Variables|Saving|GetSaveGameSlotFinalWave))
  (bind _returnvalue (SaveGame|DoesSaveGameExist _savegameslotfinalwave))
  (if _returnvalue
    (Utilities|FlowControl|Sequence
      (:then_0
        ;[0.15 0.15 0.15 0.5] Loads data
        (bind _returnvalue_2 (SaveGame|LoadGamefromSlot _savegameslotfinalwave))
        (bind _assave_game (Utilities|Casting|CastToSaveGame _returnvalue_2))
        (Utilities|FlowControl|Sequence
          (:then_0
            (Transformation|SetActorTransform (Variables|/Game/Blueprints/Saving/SaveGame.SaveGame_C|GetPlayerLocation _assave_game))
            (Class|EnemyManagerComponent|DestroyAllEnemies (Variables|Default|GetEnemy%20Management%20Component)))
          (:then_1
            (Class|GameStateLevel|SetCurrentWaveNumber (Variables|Default|GetGame%20State%20Level) (Variables|/Game/Blueprints/Saving/SaveGame.SaveGame_C|GetNumOfWaves _assave_game))
            (Development|PrintString (Utilities|String|ToString(Integer) (Variables|/Game/Blueprints/Saving/SaveGame.SaveGame_C|GetNumOfWaves _assave_game)))
            (Class|WaveManagerComponent|NewWave (Variables|Default|GetWave%20Management%20Component)))))
      (:then_1
        (Development|PrintString "Loaded Game")))
    (else
      ;[0.15 0.15 0.15 0.5] Saves if no save data has been made yet
      (SaveGame|SaveGametoSlot (Variables|Saving|GetSave%20Game%20Ref) _savegameslotfinalwave))))

(fn ChooseInputType
  (bind _aswyvern_control (Utilities|Casting|CastToWyvernControl (Game|GetPlayerController 0)))
  (if (Variables|/Game/Blueprints/WyvernControl.WyvernControl_C|GetisKBMInput _aswyvern_control)
    (Variables|Default|SetactiveSensitivity (Variables|Default|GetMSensitivity))
    (else
      (Variables|Default|SetactiveSensitivity (Variables|Default|GetCSensitivity)))))

(fn SetWyvernMaterial
  (switch int (Variables|/Game/Blueprints/GameManagers/GameManager.GameManager_C|GetwCustomizationIndex (Variables|Default|GetAs%20Game%20Manager))
    (:Default
      (Development|PrintText "Wyvern Material Index Out of Bounds"))
    (:0
      (Rendering|Material|SetMaterial (Variables|Character|GetMesh) 0 "/Game/Art/Characters/Wyvern/Materials/WyvernMaterial.WyvernMaterial"))
    (:1
      (Rendering|Material|SetMaterial (Variables|Character|GetMesh) 0 "/Game/Art/Characters/Wyvern/Materials/WyvernMaterial.WyvernMaterial"))
    (:2
      (Rendering|Material|SetMaterial (Variables|Character|GetMesh) 0 "/Game/Art/Characters/Wyvern/Materials/WyvernMaterial.WyvernMaterial"))
    (:3
      (Rendering|Material|SetMaterial (Variables|Character|GetMesh) 0 "/Game/Art/Characters/Wyvern/Materials/WyvernMaterial.WyvernMaterial"))
    (:4
      (Rendering|Material|SetMaterial (Variables|Character|GetMesh) 0 "/Game/Art/Characters/Wyvern/Materials/WyvernMaterial.WyvernMaterial"))))

(fn SetControlSensitivity
  (Default|UpdateSensitivity (Variables|Default|GetAs%20Game%20Manager))
  (CallFunction|ChooseInputType))

(fn InitializeDiveStateTimers
  (bind _returnvalue (Utilities|Time|SetTimerbyEvent (EventDispatchers|CreateEvent :!event Custom|DiveState) 0.01 true)))

(fn GetPitch
  (return (Class|KismetMathLibrary|DegAcos (Math|Vector|DotProduct (Transformation|GetActorForwardVector) (Math|Vector|VectorDown)))))

(fn InitializeHovering
  (bind _returnvalue (Utilities|Time|SetTimerbyEvent (EventDispatchers|CreateEvent :!event Custom|Hover) 0.02 true)))

(fn MovementonStart
  (bind _returnvalue (Utilities|Time|SetTimerbyEvent 0 0.02 true)))