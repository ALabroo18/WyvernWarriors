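; BP_WyvernMenu is a wyvern actor, apparently for the menu, that displays the color chosen in customization.
; On BeginPlay it casts the game instance to GameManager, caches it and binds an event to its ColorChange dispatcher.
; ChangeWyvernColor, presumably the bound handler, switches on the manager's WCustomizationIndex to set the skeletal mesh's first material to one of five wyvern skins.
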(event EventBeginPlay
  (bind _asgame_manager (Utilities|Casting|CastToGameManager (Game|GetGameInstance)))
  (Variables|Default|SetAs%20Game%20Manager _asgame_manager)
  (EventDispatchers|BindEventtoColorChange (Variables|Default|GetAs%20Game%20Manager) (EventDispatchers|CreateEvent :!event ChangeWyvernColor)))

(event Collision|EventActorBeginOverlap
  (params (OtherActor :type Actor%20Object%20Reference)))

(event EventTick
  (params (DeltaSeconds :type Float%20%28single-precision%29)))

(fn ConstructionScript)

(fn ChangeWyvernColor
  (switch int (Variables|/Game/Blueprints/GameManagers/GameManager.GameManager_C|GetwCustomizationIndex (Variables|Default|GetAs%20Game%20Manager))
    (:0
      (Rendering|Material|SetMaterial (Variables|Default|GetSkeletalMesh) 0 "/Game/Art/Characters/Wyvern/Materials/WyvernMaterial.WyvernMaterial"))
    (:1
      (Rendering|Material|SetMaterial (Variables|Default|GetSkeletalMesh) 0 "/Game/Art/Characters/Wyvern/Textures/GreenWyvern.GreenWyvern"))
    (:2
      (Rendering|Material|SetMaterial (Variables|Default|GetSkeletalMesh) 0 "/Game/Art/Characters/Wyvern/Textures/RedWyvern.RedWyvern"))
    (:3
      (Rendering|Material|SetMaterial (Variables|Default|GetSkeletalMesh) 0 "/Game/Art/Characters/Wyvern/Textures/BlackWyvern.BlackWyvern"))
    (:4
      (Rendering|Material|SetMaterial (Variables|Default|GetSkeletalMesh) 0 "/Game/Art/Characters/Wyvern/Textures/WhiteWyvern.WhiteWyvern"))))