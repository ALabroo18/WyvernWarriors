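; Manager that starts the weapon quick-time event, pairing a random weapon object with a random drop-off.
; On BeginPlay it caches the wave manager and all weapon and drop-off actors, then binds to the event bus's start-level event.
; That event sets a short one-shot timer which, unless TimeToSpawn or the final wave is set, picks the drop-off, reveals the weapon, links them and begins the QTE.
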(event Custom|WeaponQTESpawn
  ;[0.15 0.15 0.15 0.5] Spawns in WeaponQTE when called
  (bind _returnvalue (Utilities|Time|SetTimerbyFunctionName 0 "WeaponQTE" 1.0))
  (Variables|Default|SetWeaponQTEHandle _returnvalue))

(event Custom|CustomEvent_0
  (CallFunction|WeaponQTESpawn))

(event EventBeginPlay
  (bind _wavemanager (CallFunction|GetWaveManager))
  (Variables|Default|SetWave%20Management%20Component _wavemanager)
  (bind _outactors (Actor|GetAllActorsOfClass "/Game/Blueprints/WeaponQTESpawner/WeaponQTEObject.WeaponQTEObject_C"))
  (Variables|Default|SetAllWeaponObjects _outactors)
  (bind _outactors_2 (Actor|GetAllActorsOfClass "/Game/LevelDesign/BlockoutPrefabs/WeaponDropOff.WeaponDropOff_C"))
  (Variables|Default|SetAllWeaponDropOffs _outactors_2)
  (bind _eventbus (CallFunction|GetEventBus))
  (EventDispatchers|BindEventtoStartLevel _eventbus (delegate Custom|CustomEvent_0)))

(fn ConstructionScript)

(fn SetQTEtoSpawn
  (bind _output_get (Variables|Default|SetTargetWeaponObject (.OutItem (Utilities|Array|Random (Variables|Default|GetAllWeaponObjects)))))
  (Rendering|SetVisibility (Variables|/Script/Engine.Actor|GetRootComponent _output_get) true false)
  (Variables|/Game/LevelDesign/BlockoutPrefabs/WeaponDropOff.WeaponDropOff_C|SetWeapons (Variables|Default|GetTargetCauldron) _output_get)
  (Default|BeginQTE _output_get))

(fn SetVillageTarget
  (bind _output_get (Variables|Default|SetTargetCauldron (.OutItem (Utilities|Array|Random (Variables|Default|GetAllWeaponDropOffs)))))
  (Default|QTETime _output_get false)
  (return))

(fn WeaponQTE
  (if (not (or (Variables|Default|GetTimeToSpawn) (Variables|/Script/WyvernWarriors.WaveManagerComponent|GetbIsFinalWave (Variables|Default|GetWave%20Management%20Component))))
    (CallFunction|SetVillageTarget)
    (CallFunction|SetQTEtoSpawn)))