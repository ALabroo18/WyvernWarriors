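; Weapon pickup for the wyvern's QTE, hidden at its spawn point until the QTE begins and destroyed on the final wave.
; BeginQTE reveals it and starts looping timers that hide the icon once the wyvern has a weapon and scale it up with distance.
; Sphere overlap shows or hides the wyvern's QTE prompt and sets or clears its pickup reference.
; ResetQTE detaches, hides and returns it to spawn, clearing timers and restoring collision.
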(event OnComponentBeginOverlap(Sphere)
  (params (OverlappedComponent :type Primitive%20Component%20Object%20Reference) (OtherActor :type Actor%20Object%20Reference) (OtherComp :type Primitive%20Component%20Object%20Reference) (OtherBodyIndex :type Integer) (bFromSweep :type Boolean) (SweepResult :type Hit%20Result%20Structure%20%28by%20ref%29))
  (bind _asbp_wyvern (Utilities|Casting|CastToBp_wyvern OtherActor))
  (bind _output_get (Variables|Default|SetAs%20Bp%20Wyvern _asbp_wyvern))
  (Utilities|IsValid (Variables|/Game/Blueprints/Characters/Wyvern/Bp_wyvern.Bp_wyvern_C|GetWeaponPickupReference _output_get)
    (:Is%20Not%20Valid
      (Default|ShowQTE (Variables|Default|GetAs%20Bp%20Wyvern))
      (Variables|/Game/Blueprints/Characters/Wyvern/Bp_wyvern.Bp_wyvern_C|SetWeaponPickupReference (Variables|Default|GetAs%20Bp%20Wyvern) self))))

(event OnComponentEndOverlap(Sphere)
  (params (OverlappedComponent :type Primitive%20Component%20Object%20Reference) (OtherActor :type Actor%20Object%20Reference) (OtherComp :type Primitive%20Component%20Object%20Reference) (OtherBodyIndex :type Integer))
  (bind _asbp_wyvern (Utilities|Casting|CastToBp_wyvern OtherActor))
  (Default|HideQTE _asbp_wyvern)
  (Variables|/Game/Blueprints/Characters/Wyvern/Bp_wyvern.Bp_wyvern_C|SetWeaponPickupReference _asbp_wyvern 0))

(event Custom|CheckPickup
  (if (Variables|/Game/Blueprints/Characters/Wyvern/Bp_wyvern.Bp_wyvern_C|GetHasWeapon (Variables|Default|GetAs%20Bp%20Wyvern))
    (Rendering|SetVisibility (Variables|Default|GetWeaponUI) false false)))

(event Custom|ChangeImg
  (bind _returnvalue (Transformation|GetActorLocation))
  (bind _as_bp_wyvern (Variables|Default|GetAs%20Bp%20Wyvern))
  (bind _returnvalue_2 (Transformation|GetActorLocation _as_bp_wyvern))
  (bind _returnvalue_3 (Math|Vector|Distance(Vector) _returnvalue _returnvalue_2))
  ;[0.15 0.15 0.15 0.5] Continuously increasing the size of the UI image
  (bind _asweapon_qtestandin_ui (Utilities|Casting|CastToWeaponQTEStandinUI (UserInterface|GetUserWidgetObject (Variables|Default|GetWeaponUI))))
  (Variables|Default|SetAs%20Weapon%20QTEStandin%20UI _asweapon_qtestandin_ui)
  (bind _output_get (Variables|Default|SetisClose (<= _returnvalue_3 5e+04)))
  (if _output_get
    (Widget|Transform|SetRenderScale (Variables|/Game/Blueprints/WeaponQTESpawner/WeaponQTEStandinUI.WeaponQTEStandinUI_C|GetWeaponIcon (Variables|Default|GetAs%20Weapon%20QTEStandin%20UI)) (Math|Conversions|ToVector2D(Vector) (Math|Float|MapRangeClamped _returnvalue_3 5e+04 1.0 2.0 1.0)))))

(event Custom|CustomEvent
  (params (bIsFinalWave :type Boolean))
  (if bIsFinalWave
    (Actor|DestroyActor)))

(event Custom|BeginQTE
  ;[0.15 0.15 0.15 0.5] Set the UI Image and gets the Wyvern to gauge distance for later
  (EventDispatchers|BindEventtoQTEStarted (delegate Custom|BeginQTE))
  (Rendering|SetVisibility (Variables|Default|GetHolder) true true)
  (Rendering|SetVisibility (Variables|Default|GetWeaponUI) true false)
  (bind _asbp_wyvern (Utilities|Casting|CastToBp_wyvern (Game|Player|GetPlayerPawn 0)))
  (Variables|Default|SetAs%20Bp%20Wyvern _asbp_wyvern)
  (GameplayTags|AddGameplayTag (Variables|Default|GetTag%20Container) "(TagName=\"Task\")" :!class /Script/GameplayTags.BlueprintGameplayTagLibrary)
  (bind _returnvalue (Utilities|Time|SetTimerbyEvent (delegate Custom|CheckPickup) 0.2 true))
  (Variables|Default|SetIconTimer _returnvalue)
  (bind _asbp_hud (Utilities|Casting|CastToBP_HUD (HUD|GetHUD (Game|GetPlayerController 0))))
  (Variables|Default|SetStat%20HUD (Variables|/Game/Blueprints/UI/HUD/BP_HUD.BP_HUD_C|GetStatHUD _asbp_hud))
  (bind _returnvalue_2 (Utilities|Time|SetTimerbyEvent (delegate Custom|ChangeImg) 0.5 true))
  (Variables|Default|SetImageTimer _returnvalue_2))

(event EventBeginPlay
  ;[0.15 0.15 0.15 0.5] Makes sure every WeaponObject is in their spots and the player cant see them
  (Variables|Default|SetSpawnPoint (Transformation|GetWorldTransform (Variables|Default|GetDefaultSceneRoot)))
  (CallFunction|ResetQTE)
  (bind _eventbus (CallFunction|GetEventBus))
  (EventDispatchers|BindEventtoOnNewWave _eventbus (delegate Custom|CustomEvent)))

(fn ConstructionScript)

(fn ResetQTE
  (Transformation|DetachFromActor "KeepWorld" "KeepWorld" "KeepWorld")
  (Rendering|SetVisibility (Variables|Default|GetWeaponUI) false false)
  (Rendering|SetVisibility (Variables|Default|GetHolder) false true)
  (Transformation|SetActorTransform (Variables|Default|GetSpawnPoint) false true)
  (Utilities|Time|ClearandInvalidateTimerbyHandle (Variables|Default|GetIconTimer))
  (Utilities|Time|ClearandInvalidateTimerbyHandle (Variables|Default|GetImageTimer))
  (for _array_element (Actor|GetComponentsByClass "/Script/Engine.StaticMeshComponent")
    (Collision|SetCollisionEnabled _array_element "QueryAndPhysics")))