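; Egg nest actor for the egg chase event, acting as the drop-off point for a stolen egg.
; EggEventStarted spawns a spline-following grunt flagged as egg thief and attaches the level's EggPickup to it.
; SetUpTask shows the egg and a HUD theft notification.
; Overlapping the nest with a wyvern-carried egg completes the task; TaskComplete penalises the control meter if incomplete, then resets the egg and calls EggEventManager.
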(event OnComponentBeginOverlap(Sphere)
  (params (OverlappedComponent :type Primitive%20Component%20Object%20Reference) (OtherActor :type Actor%20Object%20Reference) (OtherComp :type Primitive%20Component%20Object%20Reference) (OtherBodyIndex :type Integer) (bFromSweep :type Boolean) (SweepResult :type Hit%20Result%20Structure%20%28by%20ref%29))
  ;[0.15 0.15 0.15 0.5] Logic for when egg is brought to nest
  (bind _asegg_pickup (Utilities|Casting|CastToEggPickup OtherActor))
  (if (Variables|/Game/Blueprints/EggChase/EggPickup.EggPickup_C|GetisOnWyvern _asegg_pickup)
    (Variables|Default|SetCompleted true)
    (CallFunction|TaskComplete)
    (Rendering|SetVisibility (Variables|Default|GetEggNestUI) false false)))

(event Custom|EggEventStarted
  ;[0.15 0.15 0.15 0.5] Spawns EggThief with egg around the level (rn just spawns a regular enemy with egg inside the body) (if player just instantly obtains egg, just need a model of enemy with the egg, and add the model of the egg to the player instead of attaching to enemy and unattaching and reattaching to player)
  (bind _enemymanager (CallFunction|GetEnemyManager))
  (bind (_distancealongspline _returnvalue) (Class|EnemyManagerComponent|GetGruntSpawnTransform _enemymanager (Variables|Default|GetPatrol%20Route)))
  (bind _returnvalue_2 (Class|EnemyManagerComponent|SpawnGruntEnemy _enemymanager _returnvalue _distancealongspline (Variables|Default|GetPatrol%20Route) true true))
  (bind _output_get (Variables|Default|SetEggThief _returnvalue_2))
  (Class|GruntEnemy|MoveAlongSplineOnly _returnvalue_2)
  (Variables|/Script/WyvernWarriors.GruntEnemy|SetbIsEggThief _returnvalue_2 true)
  (Transformation|AttachActorToActor (Variables|Default|GetEgg) _returnvalue_2 "None" "SnapToTarget" "KeepRelative" "KeepRelative" false))

(event EventBeginPlay
  ;[0.15 0.15 0.15 0.5] Sets variables
  (bind _returnvalue (Actor|GetActorOfClass "/Game/Blueprints/EggChase/EggEventManager.EggEventManager_C"))
  (Variables|Default|SetEggManager _returnvalue)
  (bind _enemymanager (CallFunction|GetEnemyManager))
  (Variables|Default|SetEnemy%20Management%20Component _enemymanager)
  (bind _returnvalue_2 (Actor|GetActorOfClass "/Game/Blueprints/EggChase/EggPickup.EggPickup_C"))
  (Variables|Default|SetEgg _returnvalue_2)
  (bind _wavemanager (CallFunction|GetWaveManager))
  (Variables|Default|SetWaveManager _wavemanager)
  (Rendering|SetVisibility (Variables|Default|GetEggNestUI) false false))

(fn ConstructionScript)

(fn TaskComplete
  (if (Variables|Default|GetCompleted)
    (Development|PrintString "Successful egg")
    (else
      (Class|WaveManagerComponent|ModifyControlMeterCurrent (Variables|Default|GetWaveManager) -5e+01 false)))
  (Default|ResetEgg (Variables|Default|GetEgg))
  (Default|EggEvent (Variables|Default|GetEggManager))
  (return))

(fn SetUpTask
  (bind _egg (Variables|Default|GetEgg))
  (Rendering|SetVisibility (Variables|/Game/Blueprints/EggChase/EggPickup.EggPickup_C|GetDefaultSceneRoot _egg) true true)
  (Rendering|SetVisibility (Variables|/Game/Blueprints/EggChase/EggPickup.EggPickup_C|GetEggUI _egg) true false)
  (bind _asbp_hud (Utilities|Casting|CastToBP_HUD (HUD|GetHUD (Game|GetPlayerController 0))))
  (Default|CreateNotificationPopup (Variables|/Game/Blueprints/UI/HUD/BP_HUD.BP_HUD_C|GetStatHUD _asbp_hud) " 
An enemy has stolen an egg! 
" "/Game/Art/UIArt/Egg_Icon.Egg_Icon"))