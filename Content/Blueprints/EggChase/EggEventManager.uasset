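; EggEventManager triggers the egg thief event on the level's EggNest during wave play.
; On BeginPlay it caches the WaveManagementComponent and the EggNest actor, then runs a one-shot delayed timer.
; After the delay, unless it is the final wave, SpawnEggThief calls EggEventStarted on the nest, which handles the event from there.
; The timer does not loop, despite its comment describing a repeating spawn.
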(event Custom|EggEventTimer
  ;[0.15 0.15 0.15 0.5] Spawns in event every x-x seconds
  (Utilities|FlowControl|Delay (Math|Random|RandomFloatinRange 1.0 1.0))
  (if (not (Variables|/Script/WyvernWarriors.WaveManagerComponent|GetbIsFinalWave (Variables|Default|GetWaveManager)))
    (CallFunction|SpawnEggThief)))

(event Custom|SpawnEggThief
  (Default|EggEventStarted (Variables|Default|GetEggNest)))

(event EventBeginPlay
  ;[0.15 0.15 0.15 0.5] Sets variables and starts timer
  (bind _wave_management_component (CallFunction|GetWaveManagementComponent))
  (Variables|Default|SetWaveManager _wave_management_component)
  (bind _returnvalue (Actor|GetActorOfClass "/Game/Blueprints/EggChase/EggNest.EggNest_C"))
  (Variables|Default|SetEggNest _returnvalue)
  (CallFunction|EggEventTimer))

(fn ConstructionScript)