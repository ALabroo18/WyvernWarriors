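; BP_EggThief is the thief in the egg chase, an AI-controlled actor that moves along a spline until it is killed.
; On BeginPlay it stops its AI controller's brain logic and caches the level's EggPickup, leaving movement to MoveAlongSpline on Tick.
; Damage reduces current health, and at zero or below it makes the egg jump to the player and destroys itself.
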(event EventBeginPlay
  (AI|Logic|StopLogic (Variables|/Script/AIModule.AIController|GetBrainComponent (AI|GetAIController self)) "")
  (bind _returnvalue (Actor|GetActorOfClass "/Game/Blueprints/EggChase/EggPickup.EggPickup_C"))
  (Variables|Default|SetEggPickup _returnvalue))

(event EventTick
  (params (DeltaSeconds :type Float%20%28single-precision%29))
  (Class|EnemyBase|MoveAlongSpline DeltaSeconds))

(event EventAnyDamage
  (params (Damage :type Float%20%28single-precision%29) (DamageType :type Damage%20Type%20Object%20Reference) (InstigatedBy :type Controller%20Object%20Reference) (DamageCauser :type Actor%20Object%20Reference))
  (Class|EnemyBase|ModifyCurrentHealth (* Damage -1.0))
  (if (<= (Variables|Default|GetCurrentHealth) 0.0)
    (Default|EggJumptoPlayer (Variables|Default|GetEggPickup))
    (Actor|DestroyActor)))

(fn ConstructionScript
  (|CallParentFunction))