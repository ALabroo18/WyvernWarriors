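; Blueprint function library that gives global access to the level's game framework objects and manager components.
; It casts the current game mode and game state to their Level-specific classes and returns them when valid.
; The wave manager, enemy manager and event bus getters build on the game mode getter, looking up each component by class and returning it only if valid.
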(fn GetGameModeLevel
  (bind _asbp_game_mode_level (Utilities|Casting|CastToBp_GameModeLevel (Game|GetGameMode (LocalVariables|Get__WorldContext))))
  (Utilities|IsValid _asbp_game_mode_level
    (:Is%20Valid
      (return _asbp_game_mode_level))))

(fn GetGameStateLevel
  (bind _asbp_game_state_level (Utilities|Casting|CastToBP_GameStateLevel (Game|GetGameState (LocalVariables|Get__WorldContext))))
  (Utilities|IsValid _asbp_game_state_level
    (:Is%20Valid
      (return _asbp_game_state_level))))

(fn GetWaveManagementComponent
  (bind _game_mode_level (CallFunction|GetGameModeLevel (LocalVariables|Get__WorldContext)))
  (Utilities|IsValid (Actor|GetComponentbyClass _game_mode_level "/Script/WyvernWarriors.WaveManagerComponent")
    (:Is%20Valid
      (return (Actor|GetComponentbyClass _game_mode_level "/Script/WyvernWarriors.WaveManagerComponent")))))

(fn GetEnemyManagementComponent
  (bind _game_mode_level (CallFunction|GetGameModeLevel (LocalVariables|Get__WorldContext)))
  (Utilities|IsValid (Actor|GetComponentbyClass _game_mode_level "/Script/WyvernWarriors.EnemyManagerComponent")
    (:Is%20Valid
      (return (Actor|GetComponentbyClass _game_mode_level "/Script/WyvernWarriors.EnemyManagerComponent")))))

(fn GetEventBus
  (bind _game_mode_level (CallFunction|GetGameModeLevel (LocalVariables|Get__WorldContext)))
  (Utilities|IsValid (Actor|GetComponentbyClass _game_mode_level "/Script/WyvernWarriors.EventBusComponent")
    (:Is%20Valid
      (return (Actor|GetComponentbyClass _game_mode_level "/Script/WyvernWarriors.EventBusComponent")))))