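; Level game mode that drives grunt enemy spawning and handles the level's win and lose outcomes.
; When the EventBus signals level start, a looping timer begins at the EnemyManager's runtime spawn delay, calling a function by name.
; SpawnGruntEnemy asks EnemyManager for spline-based transforms and patrol routes, skipping the final wave.
; WinLevel spawns a wyvern and shows a win screen, while LoseLevel shows a time-over widget; both pause the game.
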(event Custom|CustomEvent
  ;[0.15 0.15 0.15 0.5] Set up game mode with variables and events
  (Utilities|Time|SetTimerbyFunctionName 0 (Variables|Default|GetSpawnGruntFunctionName) (Variables|/Script/WyvernWarriors.EnemyManagerComponent|GetRuntimeGruntSpawnDelay (Variables|Default|GetEnemyManager)) true)
  (Variables|Default|SetEnemySpawnerTimer ""))

(event EventBeginPlay
  (EventDispatchers|BindEventtoStartLevel (Variables|Default|GetEventBus) (delegate Custom|CustomEvent)))

(event EventWinLevel
  ;[0.15 0.15 0.15 0.5] Load win screen
  (Game|SpawnActorfromClass "/Game/Blueprints/Characters/Wyvern/WinScreenWyvern.WinScreenWyvern_C" (Variables|Default|GetSpawn%20Transform) "Undefined" "MultiplyWithRoot" 0 0)
  (bind _returnvalue (UserInterface|CreateWidget "/Game/Blueprints/UI/WinScreen.WinScreen_C"))
  (UserInterface|Viewport|AddtoViewport _returnvalue 0)
  (Game|SetGamePaused true))

(event EventLoseLevel
  ;[0.15 0.15 0.15 0.5] Create game over screen and pause game
  (bind _returnvalue (UserInterface|CreateWidget "/Game/Blueprints/UI/MenuScreen/WB_TimeOver.WB_TimeOver_C" (Game|GetPlayerController 0)))
  (UserInterface|Viewport|AddtoViewport _returnvalue 0)
  (Variables|/Script/Engine.PlayerController|SetbShowMouseCursor (Game|GetPlayerController 0) true)
  (Input|SetInputModeUIOnly 0 _returnvalue "DoNotLock" false)
  (Game|SetGamePaused true))

(fn ConstructionScript)

(fn SpawnGruntEnemy
  (if (not (Variables|/Script/WyvernWarriors.WaveManagerComponent|GetbIsFinalWave (Variables|Default|GetWaveManager)))
    (bind (_distancealongspline _returnvalue) (Class|EnemyManagerComponent|GetGruntSpawnTransform (Variables|Default|GetEnemyManager)))
    (Class|EnemyManagerComponent|SpawnGruntEnemy (Variables|Default|GetEnemyManager) _returnvalue _distancealongspline (Class|EnemyManagerComponent|GetSpawnPatrolRoute (Variables|Default|GetEnemyManager)) false)))