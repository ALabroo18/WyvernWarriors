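; Game manager, apparently a GameInstance, holding shared state and settings for the wyvern player.
; On Init it applies display, gamma and sound mix settings, with functions to push saved volumes and sensitivity.
; It tracks kill combos on a resettable timer for the WyvernCombo component, and counts enemy fireballs to toggle the HUD warning only on state changes.
; It also manages wyvern color unlocks and selection, exposing both for save data.
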(event Custom|UpdateSensitivity
  (bind _returnvalue (Game|Player|GetPlayerPawn 0))
  ;[0.15 0.15 0.15 0.5] Update Wyvern Sensitivity Variables
  (Utilities|IsValid _returnvalue
    (:Is%20Valid
      (bind _asbp_wyvern (Utilities|Casting|CastToBp_wyvern _returnvalue))
      (Variables|/Game/Blueprints/Characters/Wyvern/Bp_wyvern.Bp_wyvern_C|SetMSensitivity _asbp_wyvern (Variables|Sensitivity|GetmouseSens))
      (Variables|/Game/Blueprints/Characters/Wyvern/Bp_wyvern.Bp_wyvern_C|SetCSensitivity _asbp_wyvern (Variables|Sensitivity|GetcontSens))
      (Default|ChooseInputType _asbp_wyvern))))

(event EventInit
  (Class|GameplayStatics|SetBaseSoundMix "/Game/Audio/MasterVolume.MasterVolume")
  (CallFunction|ApplyUserSettingsonOpen))

(fn AddComboKill
  (bind _output_get (Variables|Combo|SetcomboKills (+ (Variables|Combo|GetcomboKills) 1)))
  (if (>= _output_get (Variables|Combo|GetkillsToCombo))
    (if (Variables|Combo|GetcomboIsActive)
      (Utilities|Time|ClearandInvalidateTimerbyHandle (Variables|Combo|GetcomboTimer))
      (else
        (bind _output_get_2 (Variables|Combo|SetcomboIsActive true))
        (Variables|/Game/Blueprints/Characters/Wyvern/WyvernComponents/WyvernCombo.WyvernCombo_C|SetisComboActive (Actor|GetComponentbyClass (Game|Player|GetPlayerPawn 0) "/Game/Blueprints/Characters/Wyvern/WyvernComponents/WyvernCombo.WyvernCombo_C") _output_get_2)))
    (CallFunction|StartComboTimer)))

(fn EndCombo
  (Variables|Combo|SetcomboKills 0)
  (bind _output_get (Variables|Combo|SetcomboIsActive false))
  (Variables|/Game/Blueprints/Characters/Wyvern/WyvernComponents/WyvernCombo.WyvernCombo_C|SetisComboActive (Actor|GetComponentbyClass (Game|Player|GetPlayerPawn 0) "/Game/Blueprints/Characters/Wyvern/WyvernComponents/WyvernCombo.WyvernCombo_C") _output_get))

(fn StartComboTimer
  (bind _returnvalue (Utilities|Time|SetTimerbyFunctionName 0 "EndCombo" (Variables|Combo|GetcomboResetTime)))
  (Variables|Combo|SetcomboTimer _returnvalue))

(fn AddEnemyFireball
  (Variables|FireballTracking|SetenemyFireballCount (+ (Variables|FireballTracking|GetenemyFireballCount) 1))
  (CallFunction|CheckFireballCount))

(fn RemoveEnemyFireball
  (Variables|FireballTracking|SetenemyFireballCount (- (Variables|FireballTracking|GetenemyFireballCount) 1))
  (CallFunction|CheckFireballCount))

(fn CheckFireballCount
  (if (!= (>= (Variables|FireballTracking|GetenemyFireballCount) 1) (Variables|FireballTracking|GetenemyFireballsActive))
    (bind _output_get (Variables|FireballTracking|SetenemyFireballsActive (not (Variables|FireballTracking|GetenemyFireballsActive))))
    (Utilities|IsValid (Variables|References|GetStat%20HUD)
      (:Is%20Valid
        _)
      (:Is%20Not%20Valid
        (bind _asbp_hud (Utilities|Casting|CastToBP_HUD (HUD|GetHUD (Game|GetPlayerController 0))))
        (Variables|References|SetStat%20HUD (Variables|/Game/Blueprints/UI/HUD/BP_HUD.BP_HUD_C|GetStatHUD _asbp_hud))))
    (if _output_get
      (Default|FireballIncoming (Variables|References|GetStat%20HUD))
      (else
        (Default|NoFireballsIncoming (Variables|References|GetStat%20HUD))))))

(fn ApplyUserSettingsonOpen
  (bind _returnvalue (Settings|GetGameUserSettings))
  (Class|GameUserSettings|SetScreenResolution _returnvalue (Utilities|Struct|MakeIntPoint 1920 1080))
  (Class|GameUserSettings|ApplySettings _returnvalue true)
  (Audio|PushSoundMixModifier "/Game/Audio/MasterVolume.MasterVolume")
  (Class|GameUserSettings|LoadSettings _returnvalue false)
  (Development|ExecuteConsoleCommand (Utilities|String|ToString(Text) (Utilities|Text|FormatText "r.ToneMapperGamma {x}" (Variables|Settings|GetBrigthnessValue))) 0))

(fn ColorCheck
  (params (name :type Name))
  (if (Utilities|Array|ContainsItem (Variables|Customization|Getunlocked%20Colors) name)
    (switch name name
      (:Blue
        (Variables|Customization|SetwCustomizationIndex 0))
      (:Green
        (Variables|Customization|SetwCustomizationIndex 1))
      (:Red
        (Variables|Customization|SetwCustomizationIndex 2))
      (:Black
        (Variables|Customization|SetwCustomizationIndex 3))
      (:White
        (Variables|Customization|SetwCustomizationIndex 4)))
    (Default|CallColorChange)
    (else
      (Development|PrintText "Color Not Unlocked"))))

(fn UnlockColor
  (params (name :type Name))
  (if (Utilities|Array|ContainsItem (Variables|Customization|Getunlocked%20Colors) name)
    (Development|PrintText "adding wyvern color that is already unlocked, CARE")
    (else
      (Utilities|Array|Add (Variables|Customization|Getunlocked%20Colors) name))))

(fn SendSaveData
  (return (Variables|Customization|GetwCustomizationIndex) (Variables|Customization|Getunlocked%20Colors)))

(fn ReceiveSaveData
  (params (index :type Integer) (unlocked :type Array%20of%20Names))
  (Variables|Customization|SetwCustomizationIndex index)
  (Variables|Customization|Setunlocked%20Colors unlocked))

(fn SetSoundSettings
  (Audio|SetSoundMixClassOverride "/Game/Audio/MasterVolume.MasterVolume" "/Engine/EngineSounds/Master.Master" (Variables|Settings|GetsavedVolume) 1.0 0.0 true)
  (Audio|SetSoundMixClassOverride "/Game/Audio/MasterVolume.MasterVolume" "/Engine/EngineSounds/Music.Music" (Variables|Settings|GetsavedMusic) 1.0 1.0 true)
  (Audio|SetSoundMixClassOverride "/Game/Audio/MasterVolume.MasterVolume" "/Engine/EngineSounds/SFX.SFX" (Variables|Settings|GetsavedSFX) 1.0 1.0 true)
  (Audio|PushSoundMixModifier "/Game/Audio/MasterVolume.MasterVolume"))