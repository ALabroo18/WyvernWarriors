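; Capturable outpost that adds to or drains the wave manager's control meter every second, depending on who controls it.
; Non-final waves make it enemy-held and spawn grunts; the final wave hands it to the player.
; Radius overlaps track grunts and the wyvern: timed enemy capture scales with grunt count and pauses for the player, who reclaims it when none remain.
; Ownership changes update HUD notifications and a distance-scaled objective icon.
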(event OnComponentBeginOverlap(OutpostRadius)
  (params (OverlappedComponent :type Primitive%20Component%20Object%20Reference) (OtherActor :type Actor%20Object%20Reference) (OtherComp :type Primitive%20Component%20Object%20Reference) (OtherBodyIndex :type Integer) (bFromSweep :type Boolean) (SweepResult :type Hit%20Result%20Structure%20%28by%20ref%29))
  ;[0.15 0.15 0.15 0.5] Detects if players or enemies are within range, and starts capturing if able
  (Radius|CheckEnteringActor OtherActor))

(event OnComponentEndOverlap(OutpostRadius)
  (params (OverlappedComponent :type Primitive%20Component%20Object%20Reference) (OtherActor :type Actor%20Object%20Reference) (OtherComp :type Primitive%20Component%20Object%20Reference) (OtherBodyIndex :type Integer))
  ;[0.15 0.15 0.15 0.5] Detects if player or enemy leaves range, and stops timers if necessary
  (Radius|CheckExittingActor OtherActor))

(event Custom|PlayerCapturedNotification
  ;[0.15 0.15 0.15 0.5] Used to tell player an outpost has been reclaimed
  (Utilities|FlowControl|Delay 0.2)
  (bind _asbp_hud (Utilities|Casting|CastToBP_HUD (HUD|GetHUD (Game|GetPlayerController 0))))
  (Default|CreateNotificationPopup (Variables|/Game/Blueprints/UI/HUD/BP_HUD.BP_HUD_C|GetStatHUD _asbp_hud) " 
The outpost has been reclaimed! 
" "/Game/Art/UIArt/Outpost_Icon.Outpost_Icon"))

(event Custom|ImgScale
  (params (Distance :type Float%20%28single-precision%29))
  ;[0.15 0.15 0.15 0.5] Continiously increasing the size of the UI image
  (bind _asoutpost_ui (Utilities|Casting|CastToOutpostUI (UserInterface|GetUserWidgetObject (Variables|Default|GetOutpostUIWidget))))
  (Variables|UI|SetOutpostUI _asoutpost_ui)
  (bind _output_get (Variables|UI|SetisClose (<= Distance 5e+04)))
  (if _output_get
    (Widget|Transform|SetRenderScale (Variables|/Game/Blueprints/Outpost/OutpostUI.OutpostUI_C|GetOutpostImg (Variables|UI|GetOutpostUI)) (Math|Conversions|ToVector2D(Vector) (Math|Float|MapRangeClamped Distance 5e+04 1.0 2.0 1.0)))))

(event EventNewWave
  (params (bIsFinalWave :type Boolean))
  ;[0.15 0.15 0.15 0.5] Capture outpost for player or enemy if final wave or not.
  (if bIsFinalWave
    (Capture|PlayerCaptureOutpost)
    (Collision|SetCollisionEnabled (Variables|Default|GetOutpostRadius) "NoCollision")
    (Development|PrintString "Hello")
    (else
      (UI|EnemyControlledCosmetics)
      (Variables|Default|SetbIsPlayerControlled false)
      (Class|EnemyManagerComponent|SpawnGruntEnemiesforOutpost (Variables|Default|GetEnemy%20Management%20Component) self bIsFinalWave))))

(event EventTick
  (params (DeltaSeconds :type Float%20%28single-precision%29))
  (bind _returnvalue (Game|GetPlayerCharacter 0))
  ;[0.15 0.15 0.15 0.5] Gets distance to player and Updates Image Size every tick
  (Utilities|IsValid _returnvalue
    (:Is%20Valid
      (bind _output_get (Variables|UI|SetDistance%20to%20Player (Math|Vector|Distance(Vector) (Transformation|GetActorLocation self) (Transformation|GetActorLocation _returnvalue))))
      (CallFunction|ImgScale _output_get))))

(event EventBeginPlay
  ;[0.15 0.15 0.15 0.5] Sets outpost to enemy controlled and begins adding/subtracting to meter at game start
  (if (Variables|Default|GetbIsPlayerControlled)
    (Rendering|ToggleVisibility (Variables|Default|GetOutpostUIWidget) false)
    (bind _asbp_hud (Utilities|Casting|CastToBP_HUD (HUD|GetHUD (Game|GetPlayerController 0))))
    (Variables|UI|SetStatHUD (Variables|/Game/Blueprints/UI/HUD/BP_HUD.BP_HUD_C|GetStatHUD _asbp_hud)))
  (bind _wavemanager (CallFunction|GetWaveManager))
  (Variables|Default|SetWave%20Management%20Component _wavemanager)
  (Utilities|Time|SetTimerbyFunctionName 0 "MeterMath" 1.0 true)
  (bind _enemymanager (CallFunction|GetEnemyManager))
  (Variables|Default|SetEnemy%20Management%20Component _enemymanager))

(fn ConstructionScript)

(fn MeterMath
  (bind _wave_management_component (Variables|Default|GetWave%20Management%20Component))
  ;[0.15 0.15 0.15 0.5] Handles adding points to BattleMeter, adds if controlled by player, subtracts if not
  (if (Variables|Default|GetbIsPlayerControlled)
    (Class|WaveManagerComponent|ModifyControlMeterCurrent _wave_management_component 1.0 false)
    (else
      (Class|WaveManagerComponent|ModifyControlMeterCurrent _wave_management_component -1.0 false)))
  (return))

(fn EnemyCapturingOutpost
  ;[0.15 0.15 0.15 0.5] Gains enemy progression for enemies to capture outpost, when they get enough points, captures outpost, and notifies to change colors. Reset enemy capturing timer and progress when captured.
  (bind _output_get (Variables|Capture|SetEnemyProgression (+ (Variables|Capture|GetEnemyProgression) (Utilities|Array|Length (Variables|Default|GetGruntEnemies)))))
  (if (>= _output_get (Variables|Capture|GetPointsToCapture))
    (Capture|EnemyCaptureOutpost)
    (return)
    (else
      (return))))

(fn PlayerControlledCosmetics
  ;[0.15 0.15 0.15 0.5] Removes image for player to track objectives, and sets up text to display through StatHUD
  (Math|Integer|DecrementInt (Variables|/Game/Blueprints/UI/HUD/WBP_StatHUD.WBP_StatHUD_C|GetEnemyControlledOutposts (Variables|UI|GetStatHUD))
    (:%20%20
      (CallFunction|PlayerCapturedNotification)
      (Rendering|SetVisibility (Variables|Default|GetOutpostUIWidget) false false))))

(fn EnemyControlledCosmetics
  ;[0.15 0.15 0.15 0.5] Adds image for player to track objectives, and sets up text to display through StatHUD
  (Math|Integer|IncrementInt (Variables|/Game/Blueprints/UI/HUD/WBP_StatHUD.WBP_StatHUD_C|GetEnemyControlledOutposts (Variables|UI|GetStatHUD))
    (:%20%20
      (bind _returnvalue (Actor|GetActorOfClass "/Game/Blueprints/UI/Notifications/NotificationManager.NotificationManager_C"))
      (bind _output_get (Variables|Notifications|SetNotificationManager _returnvalue))
      (Default|EnemyOutpostNotification _output_get)
      (Rendering|SetVisibility (Variables|Default|GetOutpostUIWidget) true false))))

(fn CheckforPlayerCapture
  ;[0.15 0.15 0.15 0.5] If uncaptured, capture for player. Returns current player captured status.
  (if (not (Variables|Default|GetbIsPlayerControlled))
    (Capture|PlayerCaptureOutpost)
    (return)))

(fn EnemyApproachOutpost
  (params (EnteringGrunt :type BP%20Grunt%20Enemy%20Object%20Reference))
  ;[0.15 0.15 0.15 0.5] Adds enemies in radius and starts capture timer if possible
  (LocalVariables|SetGrunt EnteringGrunt)
  (if (and (== (Variables|/Script/WyvernWarriors.EnemyBase|GetPatrolRoute (LocalVariables|GetGrunt)) (Variables|Default|GetOutpostPatrolRoute)) (not (Utilities|Array|ContainsItem (Variables|Default|GetGruntEnemies) (LocalVariables|GetGrunt))))
    (Utilities|Array|Add (Variables|Default|GetGruntEnemies) (LocalVariables|GetGrunt)))
  (if (and (Variables|Default|GetbIsPlayerControlled) (not (Variables|Capture|GetPlayerCurrentlyInside)))
    (if (Class|KismetSystemLibrary|TimerExistsHandle (Variables|Capture|GetEnemyCaptureTimer))
      (if (Class|KismetSystemLibrary|IsTimerPausedHandle (Variables|Capture|GetEnemyCaptureTimer))
        (Utilities|Time|UnpauseTimerbyHandle (Variables|Capture|GetEnemyCaptureTimer)))
      (else
        (bind _returnvalue (Utilities|Time|SetTimerbyFunctionName 0 "EnemyCapturingOutpost" 1.0 true))
        (Variables|Capture|SetEnemyCaptureTimer _returnvalue)))
    (return)
    (else
      (return))))

(fn PlayerApproachOutpost
  ;[0.15 0.15 0.15 0.5] Sets player inside radius. If player controlled, stop enemy capture timer if timer is valid. If not, start player capture timer if it doesn't extist or unpause if it does.
  (Variables|Capture|SetPlayerCurrentlyInside true)
  (UI|HandleEnemiesInside)
  (if (Variables|Default|GetbIsPlayerControlled)
    (if (Class|KismetSystemLibrary|IsTimerPausedHandle (Variables|Capture|GetEnemyCaptureTimer))
      _
      (else
        (Utilities|Time|PauseTimerbyHandle (Variables|Capture|GetEnemyCaptureTimer))))
    (return)
    (else
      (return))))

(fn CheckEnteringActor
  (params (EnteringActor :type Actor%20Object%20Reference))
  ;[0.15 0.15 0.15 0.5] Checks if overlapped actor is wyvern or grunt
  (if (Class|GameplayStatics|ObjectIsA EnteringActor "/Game/Blueprints/Characters/Wyvern/Bp_wyvern.Bp_wyvern_C")
    (Radius|PlayerApproachOutpost)
    (else
      (bind _asbp_grunt_enemy (Utilities|Casting|CastToBP_GruntEnemy EnteringActor)
        (:then
          (Radius|EnemyApproachOutpost _asbp_grunt_enemy))
        (:CastFailed
          (return))))))

(fn CheckExittingActor
  (params (ExittingActor :type Actor%20Object%20Reference))
  ;[0.15 0.15 0.15 0.5] Stops timer and unsets player inside if player leaves detection radius. Tells grunt to return if alive, otherwise checks for still living grunts. If none alive reset enemy progression, capture outpost, and stop enemy capture timer if valid.
  (if (Class|GameplayStatics|ObjectIsA ExittingActor "/Game/Blueprints/Characters/Wyvern/Bp_wyvern.Bp_wyvern_C")
    (Variables|Capture|SetPlayerCurrentlyInside false)
    (UI|HandleEnemiesInside)
    (return)
    (else
      (bind _asbp_grunt_enemy (Utilities|Casting|CastToBP_GruntEnemy ExittingActor)
        (:then
          (Radius|GruntExitOutpost _asbp_grunt_enemy))
        (:CastFailed
          (return))))))

(fn HandleEnemiesInside
  (Default|EnemiesInsideText (Variables|UI|GetStatHUD) (Variables|Capture|GetPlayerCurrentlyInside) (Utilities|Array|Length (Variables|Default|GetGruntEnemies))))

(fn GruntExitOutpost
  (params (EnteringGrunt :type Grunt%20Enemy%20Object%20Reference%20%28by%20ref%29))
  ;[0.15 0.15 0.15 0.5] Remove grunt from array then check grunt enemy aliveness. If alive, force grunt to return to patrol route. If dead, check if any enemies left and reset progress and capture for player if noe..
  (bind _output_get (LocalVariables|SetGruntEnemy EnteringGrunt))
  (bind _output_get_2 (LocalVariables|SetGruntBlackboard (AI|GetBlackboard _output_get)))
  (Utilities|IsValid _output_get_2
    (:Is%20Valid
      (AI|Components|Blackboard|SetValueasBool (LocalVariables|GetGruntBlackboard) (LocalVariables|GetForceReturnToRouteKey) true)
      (AI|Components|Blackboard|SetValueasBool (LocalVariables|GetGruntBlackboard) (LocalVariables|GetOnPatrolRouteKey) false))
    (:Is%20Not%20Valid
      (if (Utilities|Array|IsEmpty (Variables|Default|GetGruntEnemies))
        (Variables|Capture|SetEnemyProgression 0)
        (Capture|CheckforPlayerCapture)
        (else
          (return))))))

(fn PlayerCaptureOutpost
  ;[0.15 0.15 0.15 0.5] Set cosmetics and variable to player controlled then clear outpost captured UI. Resert enemy capturing if in progress.
  (UI|PlayerControlledCosmetics)
  (Variables|Default|SetbIsPlayerControlled true)
  (Default|OutpostClear (Variables|UI|GetStatHUD))
  (Variables|Capture|SetEnemyProgression 0)
  (if (Utilities|Time|IsValidTimerHandle (Variables|Capture|GetEnemyCaptureTimer))
    (Utilities|Time|ClearandInvalidateTimerbyHandle (Variables|Capture|GetEnemyCaptureTimer))
    (return)
    (else
      (return))))

(fn EnemyCaptureOutpost
  (Variables|Default|SetbIsPlayerControlled false)
  (UI|EnemyControlledCosmetics)
  (Variables|Capture|SetEnemyProgression 0)
  (Utilities|Time|ClearandInvalidateTimerbyHandle (Variables|Capture|GetEnemyCaptureTimer)))