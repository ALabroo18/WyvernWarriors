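; Tutorial trigger that pauses the game to show the flamethrower tutorial when the third wave completes.
; BeginPlay binds to the event bus's wave-complete event, and the prompt function checks the level game state's current wave number.
; On a match it adds the tutorial widget to the viewport, pauses, then immediately calls the widget's EndFlamethrowerTutorial.
; StartFlamethrowerTutorial is an empty event.
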(event Custom|StartFlamethrowerTutorial)

(event EventBeginPlay
  (bind _eventbus (CallFunction|GetEventBus))
  (EventDispatchers|BindEventtoOnWaveComplete _eventbus (EventDispatchers|CreateEvent :!event FlamethrowerTutorialPrompt)))

(fn ConstructionScript)

(fn FlamethrowerTutorialPrompt
  (params (bIsFinalWave :type Boolean))
  (bind _game_state_level (CallFunction|GetGameStateLevel))
  (if (== (Class|GameStateLevel|GetCurrentWaveNumber _game_state_level) 3)
    (Development|PrintString "flamethrower")
    (bind _returnvalue (UserInterface|CreateWidget "/Game/Blueprints/FlamethrowerTutorial/WBP_FlamethrowerTutorial.WBP_FlamethrowerTutorial_C"))
    (bind _output_get (Variables|Default|SetRefWidgetFlamethrowerTutorial _returnvalue))
    (UserInterface|Viewport|AddtoViewport _output_get 0)
    (Game|SetGamePaused true)
    (Default|EndFlamethrowerTutorial (Variables|Default|GetRefWidgetFlamethrowerTutorial))))