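; Health pickup actor that heals the Bp_wyvern player when it enters the pickup's sphere.
; On overlap it plays a 2D sound and adds a fixed amount to the wyvern's Health, with no clamp in this graph.
; Instead of being destroyed, it teleports far below its start position, then returns after a delay to act as a respawn.
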(event OnComponentBeginOverlap(Sphere)
  (params (OverlappedComponent :type Primitive%20Component%20Object%20Reference) (OtherActor :type Actor%20Object%20Reference) (OtherComp :type Primitive%20Component%20Object%20Reference) (OtherBodyIndex :type Integer) (bFromSweep :type Boolean) (SweepResult :type Hit%20Result%20Structure%20%28by%20ref%29))
  (bind _asbp_wyvern (Utilities|Casting|CastToBp_wyvern OtherActor))
  (Audio|PlaySound2D "/Game/SFX/HealthPickup.HealthPickup" 0.2 1.0 0.0 0 0)
  (Variables|/Game/Blueprints/UI/HUD/BPA_CharacterStats.BPA_CharacterStats_C|SetHealth _asbp_wyvern (+ (Variables|/Game/Blueprints/UI/HUD/BPA_CharacterStats.BPA_CharacterStats_C|GetHealth _asbp_wyvern) 25.0))
  (Transformation|Teleport (Variables|Default|GetSisterLocation) "0, 0, 0")
  (Utilities|FlowControl|Delay 3e+01)
  (Transformation|Teleport (Variables|Default|GetInitialLocation) "0, 0, 0"))

(event Collision|EventActorBeginOverlap
  (params (OtherActor :type Actor%20Object%20Reference)))

(event EventTick
  (params (DeltaSeconds :type Float%20%28single-precision%29)))

(event EventBeginPlay
  (bind _output_get (Variables|Default|SetInitialLocation (Transformation|GetActorLocation)))
  (Variables|Default|SetSisterLocation (- _output_get "0.000000,0.000000,100000.000000")))

(fn ConstructionScript)