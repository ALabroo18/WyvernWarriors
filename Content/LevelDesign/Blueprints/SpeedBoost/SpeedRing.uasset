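; SpeedRing is a level-design boost actor that propels the player's wyvern (Bp_wyvern) when it enters the ring's box collision.
; The overlap restarts a Timeline that, on every update, overrides the wyvern's velocity with its current forward vector times BoostStrength and prints a debug string.
; A CustomEvent duplicates this logic on a second Timeline, with no binding shown here.
; An older fixed-velocity, delayed speed-reset chain is left disconnected.
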(event OnComponentBeginOverlap(BoxCollision)
  (params (OverlappedComponent :type Primitive%20Component%20Object%20Reference) (OtherActor :type Actor%20Object%20Reference) (OtherComp :type Primitive%20Component%20Object%20Reference) (OtherBodyIndex :type Integer) (bFromSweep :type Boolean) (SweepResult :type Hit%20Result%20Structure%20%28by%20ref%29))
  (bind _asbp_wyvern (Utilities|Casting|CastToBp_wyvern OtherActor))
  (Timeline|Timeline PlayFromStart
    (:Update
      (Development|PrintString "boosted")
      (Variables|/Script/Engine.MovementComponent|SetVelocity (Variables|/Script/Engine.Character|GetCharacterMovement _asbp_wyvern) (* (Transformation|GetActorForwardVector _asbp_wyvern) (Variables|Default|GetBoost%20Strength))))))

(event Custom|CustomEvent
  (params (OverlappedActor :type Actor%20Object%20Reference) (OtherActor :type Actor%20Object%20Reference))
  (bind _asbp_wyvern (Utilities|Casting|CastToBp_wyvern OtherActor))
  (Timeline|Timeline_0 PlayFromStart
    (:Update
      (Development|PrintString "boosted")
      (Variables|/Script/Engine.MovementComponent|SetVelocity (Variables|/Script/Engine.Character|GetCharacterMovement _asbp_wyvern) (* (Transformation|GetActorForwardVector _asbp_wyvern) (Variables|Default|GetBoost%20Strength))))))

(event EventBeginPlay)

(event Collision|EventActorBeginOverlap
  (params (OtherActor :type Actor%20Object%20Reference)))

(event EventTick
  (params (DeltaSeconds :type Float%20%28single-precision%29)))

(fn ConstructionScript)