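; Manager that triggers weapon QTEs at a random cauldron while waves are running.
; After a random delay from BeginPlay or a later timer call, it proceeds unless TimeToSpawn is set or the wave manager reports the final wave.
; It notifies a random Cauldron of QTE time, then passes it to a random WeaponQTESpawner to spawn the QTE.
; The timer does not loop itself.
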(event Custom|TimeToSpawnTimer
  ;[0.15 0.15 0.15 0.5] Spawns in WeaponQTE when called
  (Utilities|FlowControl|Delay (Math|Random|RandomFloatinRange 1e+01 2e+01))
  (if (not (or (Variables|Default|GetTimeToSpawn) (Variables|/Script/WyvernWarriors.WaveManagerComponent|GetbIsFinalWave (Variables|Default|GetWave%20Management%20Component))))
    (CallFunction|SetVillageTarget)
    (CallFunction|SetQTEtoSpawn)))

(event EventBeginPlay
  (bind _wavemanager (CallFunction|GetWaveManager))
  (Variables|Default|SetWave%20Management%20Component _wavemanager)
  (CallFunction|TimetoSpawnTimer))

(fn ConstructionScript)

(fn SetQTEtoSpawn
  (bind _outactors (Actor|GetAllActorsOfClass "/Game/LevelDesign/Blueprints/WeaponQTESpawner/WeaponQTESpawner.WeaponQTESpawner_C"))
  (bind _output_get (LocalVariables|SetSpawner (Utilities|Array|Get(acopy) _outactors (Math|Random|RandomIntegerinRange 0 (Utilities|Array|LastIndex _outactors)))))
  (Variables|/Game/LevelDesign/Blueprints/WeaponQTESpawner/WeaponQTESpawner.WeaponQTESpawner_C|SetCauldron _output_get (Variables|Default|GetCauldron))
  (Default|SpawnWeaponQTE (LocalVariables|GetSpawner)))

(fn SetVillageTarget
  (bind _outactors (Actor|GetAllActorsOfClass "/Game/LevelDesign/BlockoutPrefabs/Cauldron.Cauldron_C"))
  (bind _output_get (Variables|Default|SetCauldron (.OutItem (Utilities|Array|Random _outactors))))
  (Default|QTETime _output_get)
  (return))