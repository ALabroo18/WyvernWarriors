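; Capturable outpost that adds to or drains the wave control meter every second, depending on whether player or enemy holds it.
; Overlap-driven looping timers let the player's wyvern reclaim it once no grunts remain, while grunts build capture progress by headcount, paused when the wyvern enters.
; Non-final waves make it enemy-held and spawn grunts.
; Ownership changes update HUD counts, notifications and a marker widget, which Tick scales by player distance.
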(event OnComponentBeginOverlap(CharacterDetection)
  (params (OverlappedComponent :type Primitive%20Component%20Object%20Reference) (OtherActor :type Actor%20Object%20Reference) (OtherComp :type Primitive%20Component%20Object%20Reference) (OtherBodyIndex :type Integer) (bFromSweep :type Boolean) (SweepResult :type Hit%20Result%20Structure%20%28by%20ref%29))
  ;[0.15 0.15 0.15 0.5] Detects if players or enemies are within range, and starts capturing if able
  (CallFunction|CheckEnteringActor OtherActor))

(event OnComponentEndOverlap(CharacterDetection)
  (params (OverlappedComponent :type Primitive%20Component%20Object%20Reference) (OtherActor :type Actor%20Object%20Reference) (OtherComp :type Primitive%20Component%20Object%20Reference) (OtherBodyIndex :type Integer))
  ;[0.15 0.15 0.15 0.5] Detects if player or enemy leaves range, and stops timers if necessary
  (CallFunction|CheckExittingActor OtherActor))

(event Custom|PlayerCapturedNotification
  ;[0.15 0.15 0.15 0.5] Used to tell player an outpost has been reclaimed
  (Utilities|FlowControl|Delay 0.2)
  (bind _asbp_hud (Utilities|Casting|CastToBP_HUD (HUD|GetHUD (Game|GetPlayerController 0))))
  (Default|CreateNotificationPopup (Variables|/Game/Blueprints/UI/HUD/BP_HUD.BP_HUD_C|GetStatHUD _asbp_hud) " 
The outpost has been reclaimed! 
" "/Game/Art/UIArt/Outpost_Icon.Outpost_Icon"))

(event Custom|ImgScale
  (params (Distance :type Float%20%28single-precision%29))
  ;[0.15 0.15 0.15 0.5] Continiously increasing the size of the UI image
  (bind _asoutpost_ui (Utilities|Casting|CastToOutpostUI (UserInterface|GetUserWidgetObject (Variables|Default|GetOutpostUIWidget))))
  (Variables|UI|SetOutpostUI _asoutpost_ui)
  (bind _output_get (Variables|UI|SetisClose (<= Distance 5e+04)))
  (if _output_get
    (Widget|Transform|SetRenderScale (Variables|/Game/LevelDesign/Blueprints/Outpost/OutpostUI.OutpostUI_C|GetOutpostImg (Variables|UI|GetOutpostUI)) (Math|Conversions|ToVector2D(Vector) (Math|Float|MapRangeClamped Distance 5e+04 1.0 5.0 1.0)))))

(event EventNewWave
  (params (bIsFinalWave :type Boolean))
  (if (not bIsFinalWave)
    (CallFunction|EnemyControlledCosmetics)
    (Variables|Default|SetbIsPlayerControlled false)
    (Class|EnemyManagerComponent|SpawnGruntEnemiesforOutpost (Variables|Default|GetEnemy%20Management%20Component) self bIsFinalWave)))

(event EventTick
  (params (DeltaSeconds :type Float%20%28single-precision%29))
  (bind _returnvalue (Game|GetPlayerCharacter 0))
  ;[0.15 0.15 0.15 0.5] Gets distance to player and Updates Image Size every tick
  (Utilities|IsValid _returnvalue
    (:Is%20Valid
      (bind _output_get (Variables|UI|SetDistance%20to%20Player (Math|Vector|Distance(Vector) (Transformation|GetActorLocation self) (Transformation|GetActorLocation _returnvalue))))
      (CallFunction|ImgScale _output_get))))

(event EventBeginPlay
  ;[0.15 0.15 0.15 0.5] Sets outpost to enemy controlled and begins adding/subtracting to meter at game start
  (if (Variables|Default|GetbIsPlayerControlled)
    (Rendering|ToggleVisibility (Variables|Default|GetOutpostUIWidget) false)
    (bind _asbp_hud (Utilities|Casting|CastToBP_HUD (HUD|GetHUD (Game|GetPlayerController 0))))
    (Variables|UI|SetStatHUD (Variables|/Game/Blueprints/UI/HUD/BP_HUD.BP_HUD_C|GetStatHUD _asbp_hud)))
  (bind _wave_management_component (CallFunction|GetWaveManagementComponent))
  (Variables|Default|SetWave%20Management%20Component _wave_management_component)
  (Utilities|Time|SetTimerbyFunctionName 0 "MeterMath" 1.0 true)
  (bind _enemymanagementcomponent (CallFunction|GetEnemyManagementComponent))
  (Variables|Default|SetEnemy%20Management%20Component _enemymanagementcomponent))

(fn ConstructionScript)

(fn MeterMath
  (bind _wave_management_component (Variables|Default|GetWave%20Management%20Component))
  ;[0.15 0.15 0.15 0.5] Handles adding points to BattleMeter, adds if controlled by player, subtracts if not
  (if (Variables|Default|GetbIsPlayerControlled)
    (Class|WaveManagerComponent|ModifyControlMeterCurrent _wave_management_component 1.0 false)
    (else
      (Class|WaveManagerComponent|ModifyControlMeterCurrent _wave_management_component -1.0 false)))
  (return))

(fn EnemyCapturingOutpost
  ;[0.15 0.15 0.15 0.5] Gains enemy progression for enemies to capture outpost, when they get enough points, captures outpost, and notifies to change colors
  (bind _output_get (Variables|Capture|SetEnemyProgression (+ (Variables|Capture|GetEnemyProgression) (Variables|Capture|GetEnemiesInRadius))))
  (if (>= _output_get (Variables|Capture|GetPointsToCapture))
    (Variables|Default|SetbIsPlayerControlled false)
    (CallFunction|EnemyControlledCosmetics)
    (return)
    (else
      (return))))

(fn PlayerControlledCosmetics
  ;[0.15 0.15 0.15 0.5] Removes image for player to track objectives, and sets up text to display through StatHUD
  (Math|Integer|DecrementInt (Variables|/Game/Blueprints/UI/HUD/WBP_StatHUD.WBP_StatHUD_C|GetEnemyControlledOutposts (Variables|UI|GetStatHUD))
    (:%20%20
      (CallFunction|PlayerCapturedNotification)
      (Rendering|SetVisibility (Variables|Default|GetOutpostUIWidget) false false))))

(fn EnemyControlledCosmetics
  ;[0.15 0.15 0.15 0.5] Adds image for player to track objectives, and sets up text to display through StatHUD
  (Math|Integer|IncrementInt (Variables|/Game/Blueprints/UI/HUD/WBP_StatHUD.WBP_StatHUD_C|GetEnemyControlledOutposts (Variables|UI|GetStatHUD))
    (:%20%20
      (bind _returnvalue (Actor|GetActorOfClass "/Game/Blueprints/UI/Notifications/NotificationManager.NotificationManager_C"))
      (bind _output_get (Variables|Notifications|SetNotificationManager _returnvalue))
      (Default|EnemyOutpostNotification _output_get)
      (Rendering|SetVisibility (Variables|Default|GetOutpostUIWidget) true false))))

(fn CheckforPlayerCapture
  (if (== (Variables|Capture|GetEnemiesInRadius) 0)
    (CallFunction|PlayerControlledCosmetics)
    (Variables|Default|SetbIsPlayerControlled true)
    (Default|OutpostClear (Variables|UI|GetStatHUD))
    (Utilities|Time|ClearandInvalidateTimerbyHandle (Variables|Capture|GetPlayerCaptureTimer))
    (return)
    (else
      (return))))

(fn EnemyApproachOutpost
  ;[0.15 0.15 0.15 0.5] Adds enemies in radius and starts capture timer if possible
  (if (not (Variables|/Script/WyvernWarriors.WaveManagerComponent|GetbIsFinalWave (Variables|Default|GetWave%20Management%20Component)))
    (Math|Integer|IncrementInt (Variables|Capture|GetEnemiesInRadius)
      (:%20%20
        (if (and (Variables|Default|GetbIsPlayerControlled) (not (Variables|Capture|GetPlayerCurrentlyInside)))
          (if (Class|KismetSystemLibrary|TimerExistsHandle (Variables|Capture|GetEnemyCaptureTimer))
            (if (Class|KismetSystemLibrary|IsTimerPausedHandle (Variables|Capture|GetEnemyCaptureTimer))
              (Utilities|Time|UnpauseTimerbyHandle (Variables|Capture|GetEnemyCaptureTimer)))
            (else
              (bind _returnvalue (Utilities|Time|SetTimerbyFunctionName 0 "EnemyCapturingOutpost" 1.0 true))
              (Variables|Capture|SetEnemyCaptureTimer _returnvalue)))
          (return)
          (else
            _)))))
  (return))

(fn PlayerApproachOutpost
  ;[0.15 0.15 0.15 0.5] Sets player nearby, pauses enemy capture timer, and starts timer for player capture
  (Variables|Capture|SetPlayerCurrentlyInside true)
  (if (Variables|Default|GetbIsPlayerControlled)
    (if (Class|KismetSystemLibrary|IsTimerPausedHandle (Variables|Capture|GetEnemyCaptureTimer))
      _
      (else
        (Utilities|Time|PauseTimerbyHandle (Variables|Capture|GetEnemyCaptureTimer))))
    (return)
    (elif (Class|KismetSystemLibrary|TimerExistsHandle (Variables|Capture|GetPlayerCaptureTimer))
      (Utilities|Time|UnpauseTimerbyHandle (Variables|Capture|GetPlayerCaptureTimer))
      (else
        (bind _returnvalue (Utilities|Time|SetTimerbyFunctionName 0 "CheckForPlayerCapture" 1.0 true))
        (Variables|Capture|SetPlayerCaptureTimer _returnvalue)))))

(fn CheckEnteringActor
  (params (EnteringActor :type Actor%20Object%20Reference))
  ;[0.15 0.15 0.15 0.5] Checks if overlapped actor is wyvern or grunt
  (if (Class|GameplayStatics|ObjectIsA EnteringActor "/Game/Blueprints/Characters/Wyvern/Bp_wyvern.Bp_wyvern_C")
    (CallFunction|PlayerApproachOutpost)
    (elif (Class|GameplayStatics|ObjectIsA EnteringActor "/Game/Blueprints/Characters/Enemy/Grunt/BP_GruntEnemy.BP_GruntEnemy_C")
      (CallFunction|EnemyApproachOutpost)
      (else
        (return)))))

(fn CheckExittingActor
  (params (ExittingActor :type Actor%20Object%20Reference))
  ;[0.15 0.15 0.15 0.5] Checks to stop timers if relevant actor(s) leaves
  (if (Class|GameplayStatics|ObjectIsA ExittingActor "/Game/Blueprints/Characters/Wyvern/Bp_wyvern.Bp_wyvern_C")
    (Variables|Capture|SetPlayerCurrentlyInside false)
    (Utilities|Time|PauseTimerbyHandle (Variables|Capture|GetPlayerCaptureTimer))
    (elif (Class|GameplayStatics|ObjectIsA ExittingActor "/Game/Blueprints/Characters/Enemy/Grunt/BP_GruntEnemy.BP_GruntEnemy_C")
      (bind _output_get (Variables|Capture|SetEnemiesInRadius (- (Variables|Capture|GetEnemiesInRadius) 1)))
      (if (== _output_get 0)
        (Variables|Capture|SetEnemyProgression 0)
        (if (Utilities|Time|IsValidTimerHandle (Variables|Capture|GetEnemyCaptureTimer))
          (Utilities|Time|ClearandInvalidateTimerbyHandle (Variables|Capture|GetEnemyCaptureTimer))))
      (else
        (return)))))